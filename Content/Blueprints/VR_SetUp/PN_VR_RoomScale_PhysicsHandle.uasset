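; Room-scale VR pawn with floor tracking that lets the right motion controller grab objects, feel the environment and operate widgets.
; The trigger runs sphere traces to grab physics bodies with a physics handle that follows the hand each tick, or to attach destructibles until release.
; Hand collision overlaps drive haptics, controller glow and a custom widget-interaction hit result.
; Next and Previous inputs act as left mouse clicks on widgets.
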(event OnComponentEndOverlap(R_Col_Interaction)
  (params (OverlappedComponent :type Primitive%20Component%20Object%20Reference) (OtherActor :type Actor%20Object%20Reference) (OtherComp :type Primitive%20Component%20Object%20Reference) (OtherBodyIndex :type Integer))
  (bind _widgetinteraction (Variables|Default|GetWidgetInteraction))
  (Rendering|Material|SetScalarParameterValue (Variables|Default|GetMotionController%20MAT) "Emmision" 0.0 :!class /Script/Engine.MaterialInstanceDynamic)
  (Variables|Default|SetCan_Interact false)
  (Rendering|SetVisibility (Variables|Default|GetDisplay_Interaction) false false)
  (Variables|/Script/UMG.WidgetInteractionComponent|SetbEnableHitTesting _widgetinteraction true)
  (Variables|/Script/UMG.WidgetInteractionComponent|SetInteractionSource _widgetinteraction "World")
  (Audio|Components|Audio|Stop (stale OnComponentBeginOverlap(R_Col_Interaction) _returnvalue_2)))

(event OnComponentBeginOverlap(R_Col_Interaction)
  (params (OverlappedComponent :type Primitive%20Component%20Object%20Reference) (OtherActor :type Actor%20Object%20Reference) (OtherComp :type Primitive%20Component%20Object%20Reference) (OtherBodyIndex :type Integer) (bFromSweep :type Boolean) (SweepResult :type Hit%20Result%20Structure%20%28by%20ref%29))
  (bind _widgetinteraction (Variables|Default|GetWidgetInteraction))
  (bind _r_col_interaction (Variables|Default|GetR_Col_Interaction))
  (bind _returnvalue (Transformation|GetWorldLocation _r_col_interaction))
  (Rendering|Material|SetScalarParameterValue (Variables|Default|GetMotionController%20MAT) "Emmision" 0.2 :!class /Script/Engine.MaterialInstanceDynamic)
  (Rendering|SetVisibility (Variables|Default|GetDisplay_Interaction) true false)
  (Variables|/Script/UMG.WidgetInteractionComponent|SetInteractionSource _widgetinteraction "Custom")
  (Variables|/Script/UMG.WidgetInteractionComponent|SetbEnableHitTesting _widgetinteraction true)
  (bind _outhit (Collision|SphereTraceForObjects _returnvalue _returnvalue 4e+01 (Utilities|Array|MakeArray "ObjectTypeQuery2") true 0 "None"))
  (Class|WidgetInteractionComponent|SetCustomHitResult (Variables|Default|GetWidgetInteraction) _outhit)
  (if (not (Variables|Default|GetCan_Interact))
    (bind _returnvalue_2 (ForceFeedback|SpawnForceFeedbackAttached "/Game/Haptics/H_ForceFeedback_Effect_Interact_01.H_ForceFeedback_Effect_Interact_01" (Variables|Default|GetMotionController_R) "None" "0, 0, 0" "0, 0, 0" "KeepRelativeOffset" true true 1.0 0.0 "/Game/Haptics/H_ForceFeedback_Attenuation_01.H_ForceFeedback_Attenuation_01" false))
    (Variables|Default|SetCan_Interact true)))

(event OnComponentBeginOverlap(R_COLTouch_Environment)
  (params (OverlappedComponent :type Primitive%20Component%20Object%20Reference) (OtherActor :type Actor%20Object%20Reference) (OtherComp :type Primitive%20Component%20Object%20Reference) (OtherBodyIndex :type Integer) (bFromSweep :type Boolean) (SweepResult :type Hit%20Result%20Structure%20%28by%20ref%29))
  (if (not (Variables|Default|GetIs%20touching))
    (bind _returnvalue (ForceFeedback|SpawnForceFeedbackAttached "/Game/Haptics/H_ForceFeedback_Effect_Environment_01.H_ForceFeedback_Effect_Environment_01" (Variables|Default|GetMotionController_R) "None" "0, 0, 0" "0, 0, 0" "KeepRelativeOffset" false true 1.0 0.0 "/Game/Haptics/H_ForceFeedback_Attenuation_01.H_ForceFeedback_Attenuation_01" false))
    (Variables|Default|SetEnvironment%20Tocuh%20FF _returnvalue)
    (Variables|Default|SetIs%20touching true)))

(event OnComponentEndOverlap(R_COLTouch_Environment)
  (params (OverlappedComponent :type Primitive%20Component%20Object%20Reference) (OtherActor :type Actor%20Object%20Reference) (OtherComp :type Primitive%20Component%20Object%20Reference) (OtherBodyIndex :type Integer))
  (bind _r_coltouch_environment (Variables|Default|GetR_COLTouch_Environment))
  (bind _returnvalue (Transformation|GetWorldLocation _r_coltouch_environment))
  (bind _returnvalue_2 (Collision|SphereTraceForObjects _returnvalue _returnvalue 8.0 (Utilities|Array|MakeArray "ObjectTypeQuery1") true 0 "None"))
  (if (not _returnvalue_2)
    (Audio|Components|Audio|Stop (Variables|Default|GetEnvironment%20Tocuh%20FF))
    (Variables|Default|SetIs%20touching false)))

(event Custom|Pick%20Up
  (bind _hand_r (Variables|Default|GetHand_R))
  (bind _hand_r_2 (Variables|Default|GetHand_R))
  (bind _returnvalue (Transformation|GetWorldLocation _hand_r_2))
  (bind _returnvalue_2 (Transformation|GetWorldLocation _hand_r))
  (Utilities|FlowControl|Sequence
    (:then_0
      (bind (_outhit _returnvalue_3) (Collision|SphereTraceForObjects _returnvalue_2 _returnvalue_2 2e+01 (Utilities|Array|MakeArray "ObjectTypeQuery4") false 0 "None" true "(R=1.000000,G=0.000000,B=0.000000,A=1.000000)" "(R=0.000000,G=1.000000,B=0.000000,A=1.000000)" 2.0))
      (bind _output_get (Variables|Default|SetHas%20Hit _returnvalue_3))
      (Variables|Default|SetPickedUpObject (.HitComponent (Collision|BreakHitResult _outhit)))
      (Class|PhysicsHandleComponent|GrabComponentatLocation (Variables|Default|GetPhysicsHandle_L) (Variables|Default|GetPickedUpObject) "None" (Variables|Default|GetPhysicsHandle_L_Location))
      (if _output_get
        (bind _returnvalue_4 (ForceFeedback|SpawnForceFeedbackAttached "/Game/Haptics/H_ForceFeedback_Effect_Environment_01.H_ForceFeedback_Effect_Environment_01" (Variables|Default|GetMotionController_R) "None" "0, 0, 0" "0, 0, 0" "KeepRelativeOffset" true true 1.0 0.0 "/Game/Haptics/H_ForceFeedback_Attenuation_01.H_ForceFeedback_Attenuation_01" false))
        (Audio|Components|Audio|Stop _returnvalue_4)))
    (:then_1
      (bind (_outhit_2 _returnvalue_5) (Collision|SphereTraceForObjects _returnvalue _returnvalue 5.0 (Utilities|Array|MakeArray "ObjectTypeQuery6") true 0 "None" true "(R=1.000000,G=0.000000,B=0.000000,A=1.000000)" "(R=0.000000,G=1.000000,B=0.000000,A=1.000000)" 2.0))
      (bind _output_get_2 (Variables|Default|SetHas%20Hit _returnvalue_5))
      (if _output_get_2
        (bind _output_get_3 (Variables|Default|SetDes%20Object (.HitComponent (Collision|BreakHitResult _outhit_2))))
        (Physics|SetSimulatePhysics _output_get_3 false)
        (bind _returnvalue_6 (Transformation|AttachComponentToComponent _output_get_3 (Variables|Default|GetObjectHold_R) "None" "KeepWorld" "KeepWorld" "KeepWorld" true))
        (Variables|Default|SetPicked%20up%20Des _returnvalue_6)))))

(event Custom|Drop
  (bind _des_object (Variables|Default|GetDes%20Object))
  (Physics|Components|PhysicsHandle|ReleaseComponent (Variables|Default|GetPhysicsHandle_L))
  (if (Variables|Default|GetPicked%20up%20Des)
    (Transformation|DetachFromComponent _des_object "KeepWorld" "KeepWorld" "KeepWorld" true)
    (Physics|SetSimulatePhysics _des_object true)))

(event EventTick
  (params (DeltaSeconds :type Float%20%28single-precision%29))
  (Variables|Default|SetPhysicsHandle_L_Location (Transformation|GetWorldLocation (Variables|Default|GetHand_R)))
  (Physics|Components|PhysicsHandle|SetTargetLocation (Variables|Default|GetPhysicsHandle_L) (Variables|Default|GetPhysicsHandle_L_Location)))

(event EventBeginPlay
  (Class|HeadMountedDisplayFunctionLibrary|SetTrackingOrigin "Floor")
  (bind _outactors (Actor|GetAllActorsOfClass "/Game/UI/Interact/BP_InteractPanel_Touch_01.BP_InteractPanel_Touch_01_C"))
  (Variables|Default|SetInteractPanelsREF _outactors))

(event Input|ActionEvents|InputActionPrevious
  (params (Key :type Key%20Structure))
  (bind _widgetinteraction (Variables|Default|GetWidgetInteraction))
  ;[1 1 1] Enables widget interaction to mouse click
  (:Pressed
    (Class|WidgetInteractionComponent|PressPointerKey _widgetinteraction "LeftMouseButton"))
  (:Released
    (Class|WidgetInteractionComponent|ReleasePointerKey _widgetinteraction "LeftMouseButton")))

(event Input|ActionEvents|InputActionNext
  (params (Key :type Key%20Structure))
  (bind _widgetinteraction (Variables|Default|GetWidgetInteraction))
  ;[1 1 1] Enables widget interaction to mouse click
  (:Pressed
    (Class|WidgetInteractionComponent|PressPointerKey _widgetinteraction "LeftMouseButton"))
  (:Released
    (Class|WidgetInteractionComponent|ReleasePointerKey _widgetinteraction "LeftMouseButton")))

(event Input|KeyboardEvents|MotionControllerRightTrigger
  (params (Key :type Key%20Structure))
  (:Pressed
    (CallFunction|PickUp))
  (:Released
    (CallFunction|Drop)))

(fn ConstructionScript
  (bind _returnvalue (Rendering|Material|CreateDynamicMaterialInstance (Variables|Default|GetHand_R) 0 "/Game/Materials/MAT_VR_Contoller_Right.MAT_VR_Contoller_Right" "" :!class /Script/Engine.PrimitiveComponent))
  (Variables|Default|SetMotionController%20MAT _returnvalue)
  (Rendering|Material|SetScalarParameterValueonMaterials (Variables|Default|GetHand_R) "Emmision" 0.0))

(fn NewFunction0)