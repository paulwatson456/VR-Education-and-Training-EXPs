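; BP_GatherLevelAttributes resolves the current memory trial's attributes from data tables when play begins.
; It reads player, trial and speaker numbers from GI_MemSeg_03, then maps that player's trial order to get condition, list length and room count.
; It writes current and next room counts back to the game instance and looks up word lists for speakers A and B.
; Speaker hand-off and word playback logic is disconnected.
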(event EventBeginPlay
  (bind _asgi_mem_seg_03 (Utilities|Casting|CastToGI_MemSeg_03 (Game|GetGameInstance)))
  (Variables|Default|SetGI _asgi_mem_seg_03)
  ;[1 1 1] Gets data from game instance to filter data tables for level attributes
  (Variables|Default|SetPlayerID (Variables|/Game/GameMode/GI_MemSeg_03.GI_MemSeg_03_C|GetPlayerID (Variables|Default|GetGI)))
  (Variables|Default|SetTrialNumber (Variables|/Game/GameMode/GI_MemSeg_03.GI_MemSeg_03_C|GetTrialNumber (Variables|Default|GetGI)))
  (Variables|Default|SetSPA_Number (Variables|/Game/GameMode/GI_MemSeg_03.GI_MemSeg_03_C|GetSPA_Number (Variables|Default|GetGI)))
  (Variables|Default|SetSPB_Number (Variables|/Game/GameMode/GI_MemSeg_03.GI_MemSeg_03_C|GetSPB_Number (Variables|Default|GetGI)))
  ;[1 1 1] Uses PlayerID to grab the Trial Oder row and sets that information into a "map" for filtering through trial number
  (bind _returnvalue (Utilities|GetDataTableRow "/Game/DataTables/MemSeg_03_TrialOrder.MemSeg_03_TrialOrder" (Utilities|String|StringToName (Variables|Default|GetPlayerID)))
    (:then
      (bind _output_get (Variables|Default|SetTrialMap (Utilities|Map|MakeMap "T1" (.T1 (Utilities|Struct|BreakSTRUC_MemSeg_03_TrialOrder _returnvalue)) "T2" (.T2 (Utilities|Struct|BreakSTRUC_MemSeg_03_TrialOrder _returnvalue)) "T3" (.T3 (Utilities|Struct|BreakSTRUC_MemSeg_03_TrialOrder _returnvalue)) "T4" (.T4 (Utilities|Struct|BreakSTRUC_MemSeg_03_TrialOrder _returnvalue)) "T5" (.T5 (Utilities|Struct|BreakSTRUC_MemSeg_03_TrialOrder _returnvalue)) "T6" (.T6 (Utilities|Struct|BreakSTRUC_MemSeg_03_TrialOrder _returnvalue)) "T7" (.T7 (Utilities|Struct|BreakSTRUC_MemSeg_03_TrialOrder _returnvalue)) "T8" (.T8 (Utilities|Struct|BreakSTRUC_MemSeg_03_TrialOrder _returnvalue)))))
      ;[1 1 1] Uses Trial "letter" (stored in "Tial Condition") from Trial order to filter the attributes of list length and room number required for the current trial from TrialAttributes data table.
      (Variables|Default|SetTrialCondition (.Value (Utilities|Map|Find _output_get (Utilities|String|Append "T" (Utilities|String|ToString(Integer) (Variables|Default|GetTrialNumber))))))
      (bind _returnvalue_2 (Utilities|GetDataTableRow "/Game/DataTables/MemSeg_03_TrialAttributes.MemSeg_03_TrialAttributes" (Utilities|String|StringToName (Variables|Default|GetTrialCondition)))
        (:then
          (Variables|Default|SetList%20size (.ListLength (Utilities|Struct|BreakSTRUC_MemSeg_03_TrialAttributes _returnvalue_2)))
          (Variables|/Game/GameMode/GI_MemSeg_03.GI_MemSeg_03_C|SetCurrentRoomNumber (Variables|Default|GetGI) (.NumRooms (Utilities|Struct|BreakSTRUC_MemSeg_03_TrialAttributes _returnvalue_2)))
          ;[1 1 1] Uses Trial "letter" (stored in "Tial Condition") from Trial order to filter the attributes of room number required for the NEXT trial from TrialAttributes data table.
          (Variables|Default|SetNextTrialCondition (.Value (Utilities|Map|Find (Variables|Default|GetTrialMap) (Utilities|String|Append "T" (Utilities|String|ToString(Integer) (+ (Variables|Default|GetTrialNumber) 1))))))
          (bind _returnvalue_3 (Utilities|GetDataTableRow "/Game/DataTables/MemSeg_03_TrialAttributes.MemSeg_03_TrialAttributes" (Utilities|String|StringToName (Variables|Default|GetNextTrialCondition)))
            (:then
              (bind _output_get_2 (Variables|Default|SetNextRoomNumber (.NumRooms (Utilities|Struct|BreakSTRUC_MemSeg_03_TrialAttributes _returnvalue_3))))
              (Variables|/Game/GameMode/GI_MemSeg_03.GI_MemSeg_03_C|SetNextRoomNumber (Variables|Default|GetGI) _output_get_2))
            (:RowNotFound
              _))
          ;[1 1 1] Creates Map from data table to identify which word list should be used at each speaker, for each trial
          (bind _returnvalue_4 (Utilities|GetDataTableRow "/Game/DataTables/MemSeg_03_WordListOrder.MemSeg_03_WordListOrder" (Utilities|String|StringToName (Variables|Default|GetPlayerID)))
            (:then
              (Variables|Default|SetWordListOrder (Utilities|Map|MakeMap "SP1" (.SP1 (Utilities|Struct|BreakSTRUC_MemSeg_03_WordListOrder _returnvalue_4)) "SP2" (.SP2 (Utilities|Struct|BreakSTRUC_MemSeg_03_WordListOrder _returnvalue_4)) "SP3" (.SP3 (Utilities|Struct|BreakSTRUC_MemSeg_03_WordListOrder _returnvalue_4)) "SP4" (.SP4 (Utilities|Struct|BreakSTRUC_MemSeg_03_WordListOrder _returnvalue_4)) "SP5" (.SP5 (Utilities|Struct|BreakSTRUC_MemSeg_03_WordListOrder _returnvalue_4)) "SP6" (.SP6 (Utilities|Struct|BreakSTRUC_MemSeg_03_WordListOrder _returnvalue_4)) "SP7" (.SP7 (Utilities|Struct|BreakSTRUC_MemSeg_03_WordListOrder _returnvalue_4)) "SP8" (.SP8 (Utilities|Struct|BreakSTRUC_MemSeg_03_WordListOrder _returnvalue_4)) "SP9" (.SP9 (Utilities|Struct|BreakSTRUC_MemSeg_03_WordListOrder _returnvalue_4)) "SP10" (.SP10 (Utilities|Struct|BreakSTRUC_MemSeg_03_WordListOrder _returnvalue_4)) "SP11" (.SP11 (Utilities|Struct|BreakSTRUC_MemSeg_03_WordListOrder _returnvalue_4)) "SP12" (.SP12 (Utilities|Struct|BreakSTRUC_MemSeg_03_WordListOrder _returnvalue_4)) "SP13" (.SP13 (Utilities|Struct|BreakSTRUC_MemSeg_03_WordListOrder _returnvalue_4)) "SP14" (.SP14 (Utilities|Struct|BreakSTRUC_MemSeg_03_WordListOrder _returnvalue_4)) "SP15" (.SP15 (Utilities|Struct|BreakSTRUC_MemSeg_03_WordListOrder _returnvalue_4)) "SP16" (.SP16 (Utilities|Struct|BreakSTRUC_MemSeg_03_WordListOrder _returnvalue_4))))
              ;[1 1 1] Filters map of word list order by speaker ID for each trial. This then sets the word list to the correct speaker ID
              (Variables|Default|SetWordListNumberSPA (.Value (Utilities|Map|Find (Variables|Default|GetWordListOrder) (Utilities|String|Append "SP" (Utilities|String|ToString(Integer) (Variables|Default|GetSPA_Number))))))
              (Variables|Default|SetSPA_ID (Utilities|String|Append "SP" (Utilities|String|ToString(Integer) (Variables|Default|GetSPA_Number))))
              (Variables|Default|SetWordListNumberSPB (.Value (Utilities|Map|Find (Variables|Default|GetWordListOrder) (Utilities|String|Append "SP" (Utilities|String|ToString(Integer) (Variables|Default|GetSPB_Number))))))
              (Variables|Default|SetSPB_ID (Utilities|String|Append "SP" (Utilities|String|ToString(Integer) (Variables|Default|GetSPB_Number)))))))))))

(event Input|KeyboardEvents|8
  (params (Key :type Key%20Structure :default "None")))

(event Input|KeyboardEvents|9
  (params (Key :type Key%20Structure :default "None")))

(fn ConstructionScript)