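; Environment actor that loads per-participant trial attributes for a level in what appears to be a speaker and word-list experiment.
; CreateDataTable spawns a counterbalance data-table processor keyed to the game instance's PlayerID.
; AssignDataTable caches its map and trial number, then builds string lookup keys for room, speaker and start-position fields.
; Only the starting position is read from the map before the level director is notified.
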(event Custom|Set%20level%20Attributes
  (bind _leveldirectorref (Variables|Default|GetLevelDirectorREF))
  (Variables|Default|SetStartingPosition (Math|Conversions|ToInteger(Byte) (.Value (Utilities|Map|Find (Variables|Default|GetTable%20Data%20Map) (Variables|Default|GetTrialStartPosition_ID)))))
  (Utilities|IsValid _leveldirectorref
    (:Is%20Valid
      (Default|DataTableConstructed _leveldirectorref))))

(event Custom|Set%20Data%20lookup%20IDs
  (bind _column_title (CallFunction|DataSearchHeadingPreface))
  (Variables|Default|SetTrialNumberID _column_title)
  (bind _column_title_2 (CallFunction|DataSearchHeadingPreface (Variables|Default|GetRequiredRoomDataPostface)))
  (Variables|Default|SetRequiredRoomID _column_title_2)
  (bind _column_title_3 (CallFunction|DataSearchHeadingPreface (Variables|Default|GetTrialSpeaker01WordListDataPostface)))
  (Variables|Default|SetTrialSpeaker01WordList_ID _column_title_3)
  (bind _column_title_4 (CallFunction|DataSearchHeadingPreface (Variables|Default|GetTrialSpeaker02WordListDataPostface)))
  (Variables|Default|SetTrialSpeaker02WordList_ID _column_title_4)
  (bind _column_title_5 (CallFunction|DataSearchHeadingPreface (Variables|Default|GetTrialSpeaker01VoiceDataPostface)))
  (Variables|Default|SetTrialSpeaker01Voice_ID _column_title_5)
  (bind _column_title_6 (CallFunction|DataSearchHeadingPreface (Variables|Default|GetTrialSpeaker02VoiceDataPostface)))
  (Variables|Default|SetTrialSpeaker02Voice_ID _column_title_6)
  (bind _column_title_7 (CallFunction|DataSearchHeadingPreface (Variables|Default|GetTrialSpeaker01LookDataPostface)))
  (Variables|Default|SetTrialSpeaker01Look_ID _column_title_7)
  (bind _column_title_8 (CallFunction|DataSearchHeadingPreface (Variables|Default|GetTrialSpeaker02LookDataPostface)))
  (Variables|Default|SetTrialSpeaker02Look_ID _column_title_8)
  (bind _column_title_9 (CallFunction|DataSearchHeadingPreface (Variables|Default|GetTrialStartPositionDataPostface)))
  (Variables|Default|SetTrialStartPosition_ID _column_title_9)
  (CallFunction|SetLevelAttributes))

(event Custom|CreateDataTable
  (bind _returnvalue (Game|SpawnActorfromClass "/Game/Blueprints/Environment/BP_DT_Process_CounterbalanceSPK_VAR.BP_DT_Process_CounterbalanceSPK_VAR_C" (Transformation|GetActorTransform self) "Undefined" 0 0))
  (bind _output_get (Variables|Default|SetDataTable _returnvalue))
  (Variables|/Game/Blueprints/Environment/BP_DT_Process_CounterbalanceSPK_VAR.BP_DT_Process_CounterbalanceSPK_VAR_C|SetParticipantID _output_get (Utilities|String|StringToName (Variables|/Game/GameMode/GI_MemSeg_03.GI_MemSeg_03_C|GetPlayerID (Variables|Default|GetGI))))
  (Variables|/Game/Blueprints/Environment/BP_DT_Process_CounterbalanceSPK_VAR.BP_DT_Process_CounterbalanceSPK_VAR_C|SetSetLevlAttributesActor (Variables|Default|GetDataTable) self)
  (Default|GatherRowData (Variables|Default|GetDataTable)))

(event Custom|AssignDataTable
  (Variables|Default|SetTable%20Data%20Map (Variables|/Game/Blueprints/Environment/BP_DT_Process_CounterbalanceSPK_VAR.BP_DT_Process_CounterbalanceSPK_VAR_C|GetTableDataMap (Variables|Default|GetDataTable)))
  (Variables|Default|SetTrialNumber (Variables|/Game/GameMode/GI_MemSeg_03.GI_MemSeg_03_C|GetTrialNumber (Variables|Default|GetGI)))
  (CallFunction|SetDataLookupIDs))

(event EventBeginPlay
  (bind _asgi_mem_seg_03 (Utilities|Casting|CastToGI_MemSeg_03 (Game|GetGameInstance)))
  (Variables|Default|SetGI _asgi_mem_seg_03))

(fn ConstructionScript)

(fn DataSearchHeadingPreface
  (params (NewParam :type String))
  (return (Utilities|String|Append (Variables|Default|GetTrialDataPreface) (Utilities|String|ToString(Integer) (Variables|Default|GetTrialNumber)) NewParam)))