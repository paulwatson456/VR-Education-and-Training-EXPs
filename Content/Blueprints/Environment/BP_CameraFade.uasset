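; BP_CameraFade is a helper that blacks out and fades the player's view for either the FPS or VR pawn.
; SetCameraBlack, FadeIn and FadeOut run camera manager fades for PN_FPS, otherwise call VR_Pawn_03's own camera events.
; For FPS, FadeIn stays black briefly before fading to clear.
; BeginPlay enables input so key 1 triggers FadeOut, and a delayed FadeIn chain is left unconnected.
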(event Custom|FadeIn
  (bind _aspn_fps (Utilities|Casting|CastToPN_FPS (Game|Player|GetPlayerPawn 0))
    (:then
      (Utilities|IsValid _aspn_fps
        (:Is%20Valid
          (CameraFades|StartCameraFade :self (Game|GetPlayerCameraManager 0) :FromAlpha 1.0 :ToAlpha 1.0 :Duration 3.0)
          (Utilities|FlowControl|Delay 3.0)
          (CameraFades|StartCameraFade :self (Game|GetPlayerCameraManager 0) :FromAlpha 1.0 :Duration 2.0 :bHoldWhenFinished true))))
    (:CastFailed
      (bind _asvr_pawn_03 (Utilities|Casting|CastToVR_Pawn_03 (Game|Player|GetPlayerPawn 0)))
      (Default|CameraFadein _asvr_pawn_03))))

(event Custom|FadeOut
  (bind _aspn_fps (Utilities|Casting|CastToPN_FPS (Game|Player|GetPlayerPawn 0))
    (:then
      (Utilities|IsValid _aspn_fps
        (:Is%20Valid
          (CameraFades|StartCameraFade :self (Game|GetPlayerCameraManager 0) :ToAlpha 3.0 :Duration 3.0 :bHoldWhenFinished true))))
    (:CastFailed
      (bind _asvr_pawn_03 (Utilities|Casting|CastToVR_Pawn_03 (Game|Player|GetPlayerPawn 0)))
      (Default|CameraFadeOut _asvr_pawn_03))))

(event Custom|SetCameraBlack
  (bind _aspn_fps (Utilities|Casting|CastToPN_FPS (Game|Player|GetPlayerPawn 0))
    (:then
      (Utilities|IsValid _aspn_fps
        (:Is%20Valid
          (CameraFades|StartCameraFade :self (Game|GetPlayerCameraManager 0) :FromAlpha 1.0 :ToAlpha 1.0 :Duration 0.0))))
    (:CastFailed
      (bind _asvr_pawn_03 (Utilities|Casting|CastToVR_Pawn_03 (Game|Player|GetPlayerPawn 0)))
      (Default|CameraDark _asvr_pawn_03))))

(event EventBeginPlay
  (Input|EnableInput (Game|GetPlayerController 0)))

(event Input|KeyboardEvents|1
  (params (Key :type Key%20Structure :default "None"))
  (:Pressed
    (CallFunction|FadeOut)))

(fn ConstructionScript)