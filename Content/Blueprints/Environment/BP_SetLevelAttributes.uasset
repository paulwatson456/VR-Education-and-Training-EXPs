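; BP_SetLevelAttributes configures a memory-experiment level at BeginPlay from the player's ID and trial number.
; Data tables give the player's trial condition for that trial, the list length for that condition, and the player's word list per speaker slot.
; It pushes list size, speaker ID, condition and word list number into speakers SPA and SPB, then calls AddLevelData on each.
; Leftover word-playback logic is unconnected.
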(event EventBeginPlay
  (bind _spa_number (Variables|Default|GetSPA_Number))
  (bind _spb_number (Variables|Default|GetSPB_Number))
  (bind _spa (Variables|Default|GetSPA))
  (bind _spb (Variables|Default|GetSPB))
  (bind _returnvalue (Utilities|String|ToString(Integer) _spb_number))
  (bind _returnvalue_2 (Utilities|String|ToString(Integer) _spa_number))
  (bind _returnvalue_3 (Utilities|String|Append "SP" _returnvalue))
  (bind _returnvalue_4 (Utilities|String|Append "SP" _returnvalue_2))
  (bind _returnvalue_5 (Utilities|GetDataTableRow "/Game/DataTables/MemSeg_03_TrialOrder.MemSeg_03_TrialOrder" (Utilities|String|StringToName (Variables|Default|GetPlayerID)))
    (:then
      (bind _output_get (Variables|Default|SetTrialMap (Utilities|Map|MakeMap "T1" (.T1 (Utilities|Struct|BreakSTRUC_MemSeg_03_TrialOrder _returnvalue_5)) "T2" (.T2 (Utilities|Struct|BreakSTRUC_MemSeg_03_TrialOrder _returnvalue_5)) "T3" (.T3 (Utilities|Struct|BreakSTRUC_MemSeg_03_TrialOrder _returnvalue_5)) "T4" (.T4 (Utilities|Struct|BreakSTRUC_MemSeg_03_TrialOrder _returnvalue_5)) "T5" (.T5 (Utilities|Struct|BreakSTRUC_MemSeg_03_TrialOrder _returnvalue_5)) "T6" (.T6 (Utilities|Struct|BreakSTRUC_MemSeg_03_TrialOrder _returnvalue_5)) "T7" (.T7 (Utilities|Struct|BreakSTRUC_MemSeg_03_TrialOrder _returnvalue_5)) "T8" (.T8 (Utilities|Struct|BreakSTRUC_MemSeg_03_TrialOrder _returnvalue_5)))))
      (Variables|Default|SetTrialCondition (.Value (Utilities|Map|Find _output_get (Utilities|String|Append "T" (Variables|Default|GetTrialNumber)))))
      (bind _returnvalue_6 (Utilities|GetDataTableRow "/Game/DataTables/MemSeg_03_TrialAttributes.MemSeg_03_TrialAttributes" (Utilities|String|StringToName (Variables|Default|GetTrialCondition)))
        (:then
          (Variables|Default|SetList%20size (.ListLength (Utilities|Struct|BreakSTRUC_MemSeg_03_TrialAttributes _returnvalue_6)))
          (bind _returnvalue_7 (Utilities|GetDataTableRow "/Game/DataTables/MemSeg_03_WordListOrder.MemSeg_03_WordListOrder" (Utilities|String|StringToName (Variables|Default|GetPlayerID)))
            (:then
              (Variables|Default|SetWordListOrder (Utilities|Map|MakeMap "SP1" (.SP1 (Utilities|Struct|BreakSTRUC_MemSeg_03_WordListOrder _returnvalue_7)) "SP2" (.SP2 (Utilities|Struct|BreakSTRUC_MemSeg_03_WordListOrder _returnvalue_7)) "SP3" (.SP3 (Utilities|Struct|BreakSTRUC_MemSeg_03_WordListOrder _returnvalue_7)) "SP4" (.SP4 (Utilities|Struct|BreakSTRUC_MemSeg_03_WordListOrder _returnvalue_7)) "SP5" (.SP5 (Utilities|Struct|BreakSTRUC_MemSeg_03_WordListOrder _returnvalue_7)) "SP6" (.SP6 (Utilities|Struct|BreakSTRUC_MemSeg_03_WordListOrder _returnvalue_7)) "SP7" (.SP7 (Utilities|Struct|BreakSTRUC_MemSeg_03_WordListOrder _returnvalue_7)) "SP8" (.SP8 (Utilities|Struct|BreakSTRUC_MemSeg_03_WordListOrder _returnvalue_7)) "SP9" (.SP9 (Utilities|Struct|BreakSTRUC_MemSeg_03_WordListOrder _returnvalue_7)) "SP10" (.SP10 (Utilities|Struct|BreakSTRUC_MemSeg_03_WordListOrder _returnvalue_7)) "SP11" (.SP11 (Utilities|Struct|BreakSTRUC_MemSeg_03_WordListOrder _returnvalue_7)) "SP12" (.SP12 (Utilities|Struct|BreakSTRUC_MemSeg_03_WordListOrder _returnvalue_7)) "SP13" (.SP13 (Utilities|Struct|BreakSTRUC_MemSeg_03_WordListOrder _returnvalue_7)) "SP14" (.SP14 (Utilities|Struct|BreakSTRUC_MemSeg_03_WordListOrder _returnvalue_7)) "SP15" (.SP15 (Utilities|Struct|BreakSTRUC_MemSeg_03_WordListOrder _returnvalue_7)) "SP16" (.SP16 (Utilities|Struct|BreakSTRUC_MemSeg_03_WordListOrder _returnvalue_7))))
              (Variables|Default|SetWordListNumberSPA (.Value (Utilities|Map|Find (Variables|Default|GetWordListOrder) _returnvalue_4)))
              (Variables|Default|SetSPA_ID _returnvalue_4)
              (Variables|Default|SetWordListNumberSPB (.Value (Utilities|Map|Find (Variables|Default|GetWordListOrder) _returnvalue_3)))
              (Variables|Default|SetSPB_ID _returnvalue_3)
              (Variables|/Game/Blueprints/Environment/BP_WordLogic.BP_WordLogic_C|SetList%20size _spa (Variables|Default|GetList%20size))
              (Variables|/Game/Blueprints/Environment/BP_WordLogic.BP_WordLogic_C|SetSpeakerID _spa (Variables|Default|GetSPA_ID))
              (Variables|/Game/Blueprints/Environment/BP_WordLogic.BP_WordLogic_C|SetTrialCondition _spa (Variables|Default|GetTrialCondition))
              (Variables|/Game/Blueprints/Environment/BP_WordLogic.BP_WordLogic_C|SetWordListNumber _spa (Variables|Default|GetWordListNumberSPA))
              (Variables|/Game/Blueprints/Environment/BP_WordLogic.BP_WordLogic_C|SetList%20size _spb (Variables|Default|GetList%20size))
              (Variables|/Game/Blueprints/Environment/BP_WordLogic.BP_WordLogic_C|SetSpeakerID _spb (Variables|Default|GetSPB_ID))
              (Variables|/Game/Blueprints/Environment/BP_WordLogic.BP_WordLogic_C|SetTrialCondition _spb (Variables|Default|GetTrialCondition))
              (Variables|/Game/Blueprints/Environment/BP_WordLogic.BP_WordLogic_C|SetWordListNumber _spb (Variables|Default|GetWordListNumberSPB))
              (Default|AddLevelData (Variables|Default|GetSPA))
              (Default|AddLevelData (Variables|Default|GetSPB)))))))))

(event Input|KeyboardEvents|8
  (params (Key :type Key%20Structure :default "None")))

(event Input|KeyboardEvents|9
  (params (Key :type Key%20Structure :default "None")))

(fn ConstructionScript)