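; BP_LevelDirector is a level director actor that handles dialogue triggering and level transitions for a trial-based experience.
; On BeginPlay it enables input, caches the GI_MemSeg_03 game instance and finds the camera fade actor; PlayDialogue, also bound to a key, messages an audio comms Blueprint.
; LevelEnd fades out, then opens a whole or divided room by the game instance's trial state, or a named next level.
; StartChallenge is an empty stub.
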(event Custom|Level%20End
  (if (Variables|Default|GetMovingToNextTrial)
    (Default|FadeOut (Variables|Default|GetCameraFade))
    (Default|NextTrial (Variables|Default|GetGI))
    (Utilities|FlowControl|Delay 3.0)
    (if (<= (Variables|/Game/GameMode/GI_MemSeg_03.GI_MemSeg_03_C|GetNextRoomNumber (Variables|Default|GetGI)) 1)
      (Game|OpenLevel(byName) "EXP_03_Room_Whole")
      (else
        (Game|OpenLevel(byName) "EXP_03_Room_Divided")))
    (else
      (Default|FadeOut (Variables|Default|GetCameraFade))
      (Utilities|FlowControl|Delay 3.0)
      (Game|OpenLevel(byName) (Variables|Default|GetNextLevelName)))))

(event Custom|PlayDialogue
  (Class|BPIAudioComms|AudioComms(Message) (Variables|Default|GetAudioAssetsBP)))

(event Custom|Start%20Challenge)

(event EventBeginPlay
  (Input|EnableInput (Game|GetPlayerController 0))
  (bind _asgi_mem_seg_03 (Utilities|Casting|CastToGI_MemSeg_03 (Game|GetGameInstance)))
  (Variables|Default|SetGI _asgi_mem_seg_03)
  (bind _outactors (Actor|GetAllActorsOfClass "/Game/Blueprints/Environment/BP_CameraFade.BP_CameraFade_C"))
  (Variables|Default|SetCameraFade (Utilities|Array|Get(acopy) _outactors))
  (if (Utilities|DoesObjectImplementInterface (Variables|Default|GetAudioAssetsBP) "/Game/Blueprints/Interface/BP_I_AudioComms.BP_I_AudioComms_C")
    (Variables|Default|SetAudioAssetsBP (Variables|Default|GetAudioAssetsBP))))

(event Input|KeyboardEvents|2
  (params (Key :type Key%20Structure :default "None"))
  (:Pressed
    (CallFunction|PlayDialogue)))

(fn ConstructionScript)