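; Level director for the second Recall Room, scripting its sequence as either a tutorial or a recall session.
; After a short BeginPlay delay, NextEventSection picks the sequence from the game instance's RecallRoomLvlState.
; Each call advances a one-shot MultiGate through narration, a distraction task, more narration, a delayed final message and level end.
; The tutorial uses separate narration, turns UpdateData off and switches the saved state to recall before ending.
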(event Custom|TutorialLevelEvent
  (CallFunction|NextEventCheck)
  (Utilities|FlowControl|MultiGate false false -1
    (:Out%200
      (Variables|Default|SetUpdateData? false)
      (Class|INTLevelCommands|LevelEventPlayAudio(Message) (Variables|Default|GetAudioNarrationBP_01)))
    (:Out%201
      (Class|INTLevelCommands|LevelEventStartGame(Message) (Variables|Default|GetTaskDistractionBP)))
    (:Out%202
      (Class|INTLevelCommands|LevelEventPlayAudio(Message) (Variables|Default|GetAudioNarrationBP_01)))
    (:Out%203
      (Utilities|FlowControl|Delay 6e+01)
      (Class|INTLevelCommands|LevelEventPlayAudio(Message) (Variables|Default|GetAudioNarrationBP_01)))
    (:Out%204
      (Variables|/Game/GameMode/GI_MemSeg_03.GI_MemSeg_03_C|SetRecallRoomLvlState (Variables|Default|GetGI) 1)
      (CallFunction|LevelEndSPKVAR))))

(event Custom|RecallLevelEvent
  (CallFunction|NextEventCheck)
  (Utilities|FlowControl|MultiGate false false -1
    (:Out%200
      (Variables|Default|SetUpdateData? true)
      (Class|INTLevelCommands|LevelEventPlayAudio(Message) (Variables|Default|GetAudioNarrationBP_02)))
    (:Out%201
      (Class|INTLevelCommands|LevelEventStartGame(Message) (Variables|Default|GetTaskDistractionBP)))
    (:Out%202
      (Class|INTLevelCommands|LevelEventPlayAudio(Message) (Variables|Default|GetAudioNarrationBP_02)))
    (:Out%203
      (Utilities|FlowControl|Delay 6e+01)
      (Class|INTLevelCommands|LevelEventPlayAudio(Message) (Variables|Default|GetAudioNarrationBP_02)))
    (:Out%204
      (CallFunction|LevelEndSPKVAR))))

(event EventBeginPlay
  (|CallParentFunction)
  (Utilities|FlowControl|Delay 5.0)
  (CallFunction|NextEventSection))

(event Collision|EventActorBeginOverlap
  (params (OtherActor :type Actor%20Object%20Reference)))

(event EventTick
  (params (DeltaSeconds :type Float%20%28single-precision%29)))

(event EventNextEventSection
  (switch Utilities|FlowControl|Switch|SwitchonEN_Recall_LevelType_01 (Utilities|Enum|ByteToEnumEN_Recall_LevelType_01 (Variables|/Game/GameMode/GI_MemSeg_03.GI_MemSeg_03_C|GetRecallRoomLvlState (Variables|Default|GetGI)))
    (:NewEnumerator0
      (CallFunction|TutorialLevelEvent))
    (:NewEnumerator1
      (CallFunction|RecallLevelEvent))))

(fn ConstructionScript
  (|CallParentFunction))