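; Base level director for memory-segmentation experiment levels, handling fade-in, event sequencing and trial-to-trial level transitions.
; Registers itself with assigned narration and distraction-task actors, whose completion callback requests the next section, though here that step only resets a flag.
; Skip input or key 3 fades out, then opens a room chosen by a spawned attributes actor, or the title/next level using GameInstance state.
; An alternative LevelEnd routine is unwired.
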(event Custom|Level%20End
  (Default|FadeOut (Variables|Default|GetCameraFade))
  (if (Variables|Default|GetMovingToNextTrial)
    (if (Variables|Default|GetUpdateDataForNextTrial)
      (Default|NextTrial (Variables|Default|GetGI)))
    (Utilities|FlowControl|Delay 3.0)
    (if (<= (Variables|/Game/GameMode/GI_MemSeg_03.GI_MemSeg_03_C|GetNextRoomNumber (Variables|Default|GetGI)) 1)
      (Game|OpenLevel(byName) "EXP_03_Room_Whole")
      (else
        (Game|OpenLevel(byName) "EXP_03_Room_Divided")))
    (elif (Variables|/Game/GameMode/GI_MemSeg_03.GI_MemSeg_03_C|GetMaxTrialsCompleted (Variables|Default|GetGI))
      (Variables|/Game/GameMode/GI_MemSeg_03.GI_MemSeg_03_C|SetTitleLvlState (Variables|Default|GetGI) 4)
      (Game|OpenLevel(byName) (Variables|Default|GetTitleLevelName))
      (else
        (Variables|/Game/GameMode/GI_MemSeg_03.GI_MemSeg_03_C|SetTitleLvlState (Variables|Default|GetGI) (Variables|Default|GetTitleLevelStateOnLevelEnd))
        (Utilities|FlowControl|Delay 3.0)
        (Game|OpenLevel(byName) (Variables|Default|GetNextLevelName))))))

(event Custom|Level%20End%20SPK%20VAR
  (Default|FadeOut (Variables|Default|GetCameraFade))
  (Utilities|FlowControl|Delay 3.5)
  (if (Variables|Default|GetMovingToNextTrial)
    (bind _returnvalue (Game|SpawnActorfromClass "/Game/Blueprints/Environment/BP_SetLevelAttributes_SPK_VAR.BP_SetLevelAttributes_SPK_VAR_C" (Transformation|GetActorTransform self) "Undefined" 0 0))
    (Utilities|FlowControl|Delay 0.2)
    (switch string (.Value (Utilities|Map|Find (Variables|/Game/Blueprints/Environment/BP_SetLevelAttributes_SPK_VAR.BP_SetLevelAttributes_SPK_VAR_C|GetTable%20Data%20Map _returnvalue) (Variables|/Game/Blueprints/Environment/BP_SetLevelAttributes_SPK_VAR.BP_SetLevelAttributes_SPK_VAR_C|GetRequiredRoomID _returnvalue)))
      (:A
        (Game|OpenLevel(byName) "MemSeg_03_SP_var_Rm_A"))
      (:B
        (Game|OpenLevel(byName) "MemSeg_03_SP_var_Rm_B"))
      (:C
        (Game|OpenLevel(byName) "MemSeg_03_SP_var_Rm_C"))
      (:D
        (Game|OpenLevel(byName) "MemSeg_03_SP_var_Rm_D")))
    (elif (Variables|/Game/GameMode/GI_MemSeg_03.GI_MemSeg_03_C|GetMaxTrialsCompleted (Variables|Default|GetGI))
      (Variables|/Game/GameMode/GI_MemSeg_03.GI_MemSeg_03_C|SetTitleLvlState (Variables|Default|GetGI) 4)
      (Game|OpenLevel(byName) (Variables|Default|GetTitleLevelName))
      (else
        (Variables|/Game/GameMode/GI_MemSeg_03.GI_MemSeg_03_C|SetTitleLvlState (Variables|Default|GetGI) (Variables|Default|GetTitleLevelStateOnLevelEnd))
        (Utilities|FlowControl|Delay 3.0)
        (Game|OpenLevel(byName) (Variables|Default|GetNextLevelName))))))

(event Custom|Next%20Event%20Section
  ;[1 1 1] Event sequence chain logic. content for each step in the chain is handled by actors assigned public variables
  (CallFunction|NextEventCheck))

(event EventBeginPlay
  (Utilities|InitialiseCommonVariables)
  (Default|Fadein (Variables|Default|GetCameraFade))
  (Utilities|FlowControl|Delay (Variables|Default|GetDelayEventStart))
  (CallFunction|NextEventSection))

(event EventLevelEventComplete
  ;[1 1 1] Inteface callback from actors taking part in the event chain to inform that chain compoent is completed and the next event section will be called.
  (Variables|Default|SetCurrentEventSectionFinished? true)
  (CallFunction|NextEventSection))

(event Input|ActionEvents|InputActionSkipLevel
  (params (Key :type Key%20Structure :default "None"))
  (:Pressed
    (CallFunction|LevelEndSPKVAR)))

(event Input|KeyboardEvents|3
  (params (Key :type Key%20Structure :default "None"))
  (:Pressed
    (CallFunction|LevelEndSPKVAR)))

(fn ConstructionScript)

(fn NextEventCheck
  (if (Variables|Default|GetCurrentEventSectionFinished?)
    (Variables|Default|SetCurrentEventSectionFinished? false)))