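; Dialogue audio actor for the tutorial room that plays voice lines for comms, the ball game and a countdown.
; Three events each play from their own sound array, sharing an AudioPlaying lock held for clip length plus two seconds.
; Finished comms lines advance the track and send the level director a section-end message; ball lines set BallGameStarted.
; Countdown calls made during playback skip their line by advancing the index.
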(event Custom|BallDiag
  (bind _ballgamesoundarray (Variables|Default|GetBallGameSoundArray))
  (bind _ballgameaudiotracknumber (Variables|Default|GetBallGameAudioTrackNumber))
  (bind _output (Utilities|Array|Get(acopy) _ballgamesoundarray _ballgameaudiotracknumber))
  (if (not (Variables|Default|GetAudioPlaying?))
    (Audio|PlaySoundatLocation _output "0, 0, 0" "0, 0, 0" 1.0 1.0 0.0 0 0 0)
    (Variables|Default|SetAudioPlaying? true)
    (Utilities|FlowControl|Delay (+ (Variables|/Script/Engine.SoundBase|GetDuration _output) 2.0))
    (Variables|Default|SetAudioPlaying? false)
    (bind _asbp_lvl_dir_tutorial_room (Utilities|Casting|CastToBP_LvlDir_TutorialRoom (Variables|Default|GetLevelDirector)))
    (Variables|/Game/Blueprints/Environment/BP_LvlDir_TutorialRoom.BP_LvlDir_TutorialRoom_C|SetBallGameStarted _asbp_lvl_dir_tutorial_room true)))

(event Custom|Countdown%20Diag
  (if (Variables|Default|GetAudioPlaying?)
    (Variables|Default|SetCountdownAudioTrackNumber (+ (Variables|Default|GetCountdownAudioTrackNumber) 1))
    (else
      (Audio|PlaySoundatLocation (Utilities|Array|Get(acopy) (Variables|Default|GetCountdownSoundArray) (Variables|Default|GetCountdownAudioTrackNumber)) "0, 0, 0" "0, 0, 0" 1.0 1.0 0.0 0 0 0)
      (Variables|Default|SetAudioPlaying? true)
      (Utilities|FlowControl|Delay (+ (Variables|/Script/Engine.SoundBase|GetDuration (Utilities|Array|Get(acopy) (Variables|Default|GetCountdownSoundArray) (Variables|Default|GetCountdownAudioTrackNumber))) 2.0))
      (Variables|Default|SetAudioPlaying? false)
      (Variables|Default|SetCountdownAudioTrackNumber (+ (Variables|Default|GetCountdownAudioTrackNumber) 1)))))

(event EventBeginPlay
  (bind _outactors (Actor|GetAllActorsOfClass "/Game/Blueprints/Environment/BP_LvlDir_TutorialRoom.BP_LvlDir_TutorialRoom_C"))
  (Variables|Default|SetLevelDirector (Utilities|Array|Get(acopy) _outactors)))

(event EventAudioComms
  (if (not (Variables|Default|GetAudioPlaying?))
    (Audio|PlaySoundatLocation (Utilities|Array|Get(acopy) (Variables|Default|GetSoundArray) (Variables|Default|GetAudioTrackNumber)) "0, 0, 0" "0, 0, 0" 1.0 1.0 0.0 0 0 0)
    (Variables|Default|SetAudioPlaying? true)
    (Utilities|FlowControl|Delay (+ (Variables|/Script/Engine.SoundBase|GetDuration (Utilities|Array|Get(acopy) (Variables|Default|GetSoundArray) (Variables|Default|GetAudioTrackNumber))) 2.0))
    (Variables|Default|SetAudioPlaying? false)
    (Variables|Default|SetAudioTrackNumber (+ (Variables|Default|GetAudioTrackNumber) 1))
    (Class|BPIEventSectionEnd|EventSectionEnd(Message) (Variables|Default|GetLevelDirector))))

(fn ConstructionScript)