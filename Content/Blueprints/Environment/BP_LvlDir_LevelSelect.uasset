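; Level director for an experiment's title and recall levels, choosing tutorial, recall or trial-start flow from the game instance's TitleLvlState.
; BeginPlay spawns that flow's actors: power base and player-facing UI, or dialogue audio and maths distraction task.
; MultiGates advance the event chain as spawned actors report completion, leaving each step's content to those actors.
; LevelEnd fades the camera and opens the next trial room or named level.
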(event Custom|Level%20End
  (if (Variables|Default|GetMovingToNextTrial)
    (Default|FadeOut (Variables|Default|GetCameraFade))
    (Default|NextTrial (Variables|Default|GetGI))
    (Utilities|FlowControl|Delay 3.0)
    (if (<= (Variables|/Game/GameMode/GI_MemSeg_03.GI_MemSeg_03_C|GetNextRoomNumber (Variables|Default|GetGI)) 1)
      (Game|OpenLevel(byName) "EXP_03_Room_Whole")
      (else
        (Game|OpenLevel(byName) "EXP_03_Room_Divided")))
    (else
      (Default|FadeOut (Variables|Default|GetCameraFade))
      (Utilities|FlowControl|Delay 3.0)
      (Game|OpenLevel(byName) (Variables|Default|GetNextLevelName)))))

(event Custom|DestroyUI
  (Actor|DestroyActor (Variables|Default|GetCurrentUI))
  (Variables|Default|SetUI_SequenceNumber (+ (Variables|Default|GetUI_SequenceNumber) 1))
  (Utilities|FlowControl|Delay 0.5)
  (CallFunction|SpawnUI))

(event Custom|SpawnUI
  (bind _powerref (Variables|Default|GetPowerREF))
  (bind _returnvalue (Transformation|GetActorLocation _powerref))
  (Variables|Default|SetCurrentUIClass (Utilities|Array|Get(acopy) (Variables|Default|GetUI_Sequence) (Variables|Default|GetUI_SequenceNumber)))
  (bind _returnvalue_2 (Game|SpawnActorfromClass (Variables|Default|GetCurrentUIClass) (Math|Conversions|ToTransform(Vector) (Math|Vector|MakeVector (+ (.x _returnvalue) 5e+01) (.y _returnvalue) (- (Variables|/Script/Engine.Pawn|GetBaseEyeHeight (Game|Player|GetPlayerPawn 0)) 25.0))) "Undefined" 0 0))
  (bind _output_get (Variables|Default|SetCurrentUI _returnvalue_2))
  (Transformation|SetActorRotation _output_get (Math|Rotator|MakeRotator 0.0 0.0 (.yaw (Math|Rotator|FindLookatRotation (Transformation|GetActorLocation _output_get) (Transformation|GetActorLocation (Game|Player|GetPlayerPawn 0))))))
  (bind _asbp_power_manager_01 (Utilities|Casting|CastToBP_PowerManager_01 (Variables|Default|GetPowerREF)))
  (bind _output_get_2 (Variables|/Game/Blueprints/Environment/BP_PowerManager_01.BP_PowerManager_01_C|SetSubjectToPower_01 _asbp_power_manager_01 _output_get))
  (Utilities|IsValid _output_get_2
    (:Is%20Valid
      (bind _asbp_start_game (Utilities|Casting|CastToBP_StartGame _output_get))
      (Variables|/Game/UI/3D_UI/BP_StartGame.BP_StartGame_C|SetLevelDirectorREF _asbp_start_game self))))

(event Custom|Next%20Event%20Section
  ;[1 1 1] Event sequence chain logic. content for each step in the chain is handled by separate actors
  (if (Variables|Default|GetCurrentEventSectionFinished?)
    (Variables|Default|SetCurrentEventSectionFinished? false)
    (switch Utilities|FlowControl|Switch|SwitchonEN_LevelType_01 (Utilities|Enum|ByteToEnumEN_LevelType_01 (Variables|Default|GetLevelType))
      (:NewEnumerator0
        (Utilities|FlowControl|MultiGate false false -1
          (:Out%200
            (CallFunction|SpawnUI))
          (:Out%201
            (CallFunction|DestroyUI))))
      (:NewEnumerator1
        (Utilities|FlowControl|MultiGate false false -1
          (:Out%200
            (Utilities|FlowControl|Delay 5.0)
            (Class|BPIAudioComms|AudioComms(Message) (Variables|Default|GetAudioAssetsBP)))
          (:Out%201
            (Class|BPIChallengeComms|ChallengeComms(Message) (Variables|Default|GetChallengeBP)))
          (:Out%202
            (Class|BPIAudioComms|AudioComms(Message) (Variables|Default|GetAudioAssetsBP)))
          (:Out%203
            (Class|BPIAudioComms|AudioComms(Message) (Variables|Default|GetAudioAssetsBP)))
          (:Out%204
            (CallFunction|LevelEnd))))
      (:NewEnumerator2
        (CallFunction|LevelEnd))
      (:NewEnumerator4
        (Utilities|FlowControl|MultiGate false false -1
          (:Out%200
            (Utilities|FlowControl|Delay 5.0)
            (Class|BPIAudioComms|AudioComms(Message) (Variables|Default|GetAudioAssetsBP)) ; Introduction to distractor task
          )
          (:Out%201
            (Class|BPIChallengeComms|ChallengeComms(Message) (Variables|Default|GetChallengeBP)) ; Activate distarctor task
          )
          (:Out%202
            (Class|BPIAudioComms|AudioComms(Message) (Variables|Default|GetAudioAssetsBP)) ; Challenge complete dialogue and recall instruction
          )
          (:Out%203
            (Class|BPIAudioComms|AudioComms(Message) (Variables|Default|GetAudioAssetsBP)) ; recall complete and next instructions
          )
          (:Out%204
            (Variables|Default|SetMovingToNextTrial false)
            (Variables|/Game/GameMode/GI_MemSeg_03.GI_MemSeg_03_C|SetTitleLvlState (Variables|Default|GetGI) 2)
            (Variables|Default|SetNextLevelName "EXP_03_Title_02")
            (CallFunction|LevelEnd)))))))

(event EventBeginPlay
  (Input|EnableInput (Game|GetPlayerController 0))
  (bind _asgi_mem_seg_03 (Utilities|Casting|CastToGI_MemSeg_03 (Game|GetGameInstance)))
  (Variables|Default|SetGI _asgi_mem_seg_03)
  (bind _outactors (Actor|GetAllActorsOfClass "/Game/Blueprints/Environment/BP_CameraFade.BP_CameraFade_C"))
  (Variables|Default|SetCameraFade (Utilities|Array|Get(acopy) _outactors))
  (Variables|Default|SetLevelType (Variables|/Game/GameMode/GI_MemSeg_03.GI_MemSeg_03_C|GetTitleLvlState (Variables|Default|GetGI)))
  (switch Utilities|FlowControl|Switch|SwitchonEN_LevelType_01 (Utilities|Enum|ByteToEnumEN_LevelType_01 (Variables|Default|GetLevelType))
    (:NewEnumerator0
      (bind _returnvalue (Game|SpawnActorfromClass "/Game/Blueprints/Environment/BP_PowerManager_01.BP_PowerManager_01_C" (Math|Transform|MakeTransform "20.000000,30.000000,-110.000000" "0.000000,180.000000,0.000000") "Undefined" 0 0))
      (Variables|Default|SetPowerREF _returnvalue)
      (Game|SpawnActorfromClass "/Game/UI/3D_UI/3DUI_FloorIcon_01.3DUI_FloorIcon_01_C" (Math|Transform|MakeTransform "20.000000,30.000000,-110.000000" "0.000000,180.000000,0.000000") "Undefined" 0 0)
      (CallFunction|NextEventSection))
    (:NewEnumerator1
      (bind _returnvalue_2 (Game|SpawnActorfromClass "/Game/Blueprints/Environment/BP_Diag_RecallRoom_01.BP_Diag_RecallRoom_01_C" (Transformation|GetActorTransform (Variables|Default|GetSpawnLocation_01)) "Undefined" 0 0))
      (Variables|Default|SetAudioAssetsBP _returnvalue_2)
      (bind _returnvalue_3 (Game|SpawnActorfromClass "/Game/Blueprints/DistractionTask/BP_DistractionTask_Maths_02.BP_DistractionTask_Maths_02_C" (Transformation|GetActorTransform (Variables|Default|GetSpawnLocation_01)) "Undefined" 0 0))
      (Variables|Default|SetChallengeBP _returnvalue_3)
      (Variables|/Game/GameMode/GI_MemSeg_03.GI_MemSeg_03_C|SetTitleLvlState (Variables|Default|GetGI) 2)
      (Variables|Default|SetMovingToNextTrial false)
      (CallFunction|NextEventSection))
    (:NewEnumerator2
      (bind _returnvalue_4 (Game|SpawnActorfromClass "/Game/Blueprints/Environment/BP_PowerManager_01.BP_PowerManager_01_C" (Math|Transform|MakeTransform (Variables|Default|GetPowerBase_LOC) "0.000000,180.000000,0.000000") "Undefined" 0 0))
      (Variables|Default|SetPowerREF _returnvalue_4)
      (bind _returnvalue_5 (Game|SpawnActorfromClass "/Game/UI/3D_UI/BP_StartTrial.BP_StartTrial_C" (Math|Conversions|ToTransform(Vector) (Math|Vector|MakeVector (+ (.x (Transformation|GetActorLocation (Variables|Default|GetPowerREF))) 5e+01) (.y (Transformation|GetActorLocation (Variables|Default|GetPowerREF))) (- (Variables|/Script/Engine.Pawn|GetBaseEyeHeight (Game|Player|GetPlayerPawn 0)) 25.0))) "Undefined" 0 0))
      (bind _output_get (Variables|Default|SetCurrentUI _returnvalue_5))
      (Transformation|SetActorRotation _output_get (Math|Rotator|MakeRotator 0.0 0.0 (.yaw (Math|Rotator|FindLookatRotation (Transformation|GetActorLocation _output_get) (Transformation|GetActorLocation (Game|Player|GetPlayerPawn 0))))))
      (bind _asbp_power_manager_01 (Utilities|Casting|CastToBP_PowerManager_01 (Variables|Default|GetPowerREF)))
      (Variables|/Game/Blueprints/Environment/BP_PowerManager_01.BP_PowerManager_01_C|SetSubjectToPower_01 _asbp_power_manager_01 _output_get)
      (bind _asbp_start_trial (Utilities|Casting|CastToBP_StartTrial _output_get))
      (Variables|/Game/UI/3D_UI/BP_StartTrial.BP_StartTrial_C|SetLevelDirectorREF _asbp_start_trial self))
    (:NewEnumerator4
      (bind _returnvalue_6 (Game|SpawnActorfromClass "/Game/Blueprints/Environment/BP_Diag_RecallRoom_TUT_01.BP_Diag_RecallRoom_TUT_01_C" (Transformation|GetActorTransform (Variables|Default|GetSpawnLocation_01)) "Undefined" 0 0))
      (Variables|Default|SetAudioAssetsBP _returnvalue_6)
      (bind _returnvalue_7 (Game|SpawnActorfromClass "/Game/Blueprints/DistractionTask/BP_DistractionTask_Maths_02.BP_DistractionTask_Maths_02_C" (Transformation|GetActorTransform (Variables|Default|GetSpawnLocation_01)) "Undefined" 0 0))
      (Variables|Default|SetChallengeBP _returnvalue_7)
      (CallFunction|NextEventSection))))

(event EventChallengeComms
  (CallFunction|EventSectionEnd))

(event EventEventSectionEnd
  ;[1 1 1] Event sequence chain logic. content for each step in the chain is handled by separate actors
  ;;[1 1 1] Inteface callback from actors taking part in the event chain to inform that chain compoent is completed and the next event section will be called.
  (Development|PrintString "event fired")
  (Variables|Default|SetCurrentEventSectionFinished? true)
  (CallFunction|NextEventSection))

(fn ConstructionScript)