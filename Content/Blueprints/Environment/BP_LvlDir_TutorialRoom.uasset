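; Level director for the tutorial room of what appears to be a memory experiment, running timed dialogue and the exit to the next level.
; A gated MultiGate steps through two comms messages on the dialogue actor, advanced by EventSectionEnd callbacks from chain actors.
; BeginPlay timers trigger countdown dialogue, then LevelEnd fades the camera and opens either the named next level or a whole/divided room chosen through the game instance's trial state.
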(event Custom|Level%20End
  (CallFunction|Countdown)
  (Utilities|FlowControl|Delay 5.0)
  (if (Variables|Default|GetMovingToNextTrial)
    (Default|FadeOut (Variables|Default|GetCameraFade))
    (Default|NextTrial (Variables|Default|GetGI))
    (Utilities|FlowControl|Delay 3.0)
    (if (<= (Variables|/Game/GameMode/GI_MemSeg_03.GI_MemSeg_03_C|GetNextRoomNumber (Variables|Default|GetGI)) 1)
      (Game|OpenLevel(byName) "EXP_03_Room_Whole")
      (else
        (Game|OpenLevel(byName) "EXP_03_Room_Divided")))
    (else
      (Default|FadeOut (Variables|Default|GetCameraFade))
      (Utilities|FlowControl|Delay 3.0)
      (Game|OpenLevel(byName) (Variables|Default|GetNextLevelName)))))

(event Custom|Start%20Ball%20Game
  (if (not (Variables|Default|GetBallGameStarted))
    (bind _asbp_diag_tutorial_room_01 (Utilities|Casting|CastToBP_Diag_TutorialRoom_01 (Variables|Default|GetAudioAssetsBP)))
    (Default|BallDiag _asbp_diag_tutorial_room_01)))

(event Custom|Countdown
  (bind _asbp_diag_tutorial_room_01 (Utilities|Casting|CastToBP_Diag_TutorialRoom_01 (Variables|Default|GetAudioAssetsBP)))
  (Default|CountdownDiag _asbp_diag_tutorial_room_01))

(event Custom|Countdown%2001
  (CallFunction|Countdown))

(event Custom|Next%20Dialogue%20Section
  ;[1 1 1] Event sequence chain logic. content for each step in the chain is handled by separate actors
  (if (Variables|Default|GetCurrentEventSectionFinished?)
    (Variables|Default|SetCurrentEventSectionFinished? false)
    (Utilities|FlowControl|MultiGate false false -1
      (:Out%200
        (Class|BPIAudioComms|AudioComms(Message) (Variables|Default|GetAudioAssetsBP)) ; Introduction to distractor task
      )
      (:Out%201
        (Class|BPIAudioComms|AudioComms(Message) (Variables|Default|GetAudioAssetsBP)) ; Challenge complete dialogue and recall instruction
      ))))

(event Custom|Countdown%2002
  (CallFunction|Countdown))

(event EventBeginPlay
  (Utilities|Time|SetTimerbyEvent (delegate Custom|Countdown%2001) 3e+01)
  (Utilities|Time|SetTimerbyEvent (delegate Custom|Countdown%2002) 4e+01)
  (Utilities|Time|SetTimerbyEvent (delegate Custom|Level%20End) 5e+01)
  (Input|EnableInput (Game|GetPlayerController 0))
  (bind _asgi_mem_seg_03 (Utilities|Casting|CastToGI_MemSeg_03 (Game|GetGameInstance)))
  (Variables|Default|SetGI _asgi_mem_seg_03)
  (bind _outactors (Actor|GetAllActorsOfClass "/Game/Blueprints/Environment/BP_CameraFade.BP_CameraFade_C"))
  (Variables|Default|SetCameraFade (Utilities|Array|Get(acopy) _outactors))
  (bind _outactors_2 (Actor|GetAllActorsOfClass "/Game/Blueprints/Environment/BP_Diag_TutorialRoom_01.BP_Diag_TutorialRoom_01_C"))
  (Variables|Default|SetAudioAssetsBP (Utilities|Array|Get(acopy) _outactors_2))
  (Utilities|FlowControl|Delay 5.0)
  (CallFunction|NextDialogueSection))

(event EventEventSectionEnd
  ;[1 1 1] Event sequence chain logic. content for each step in the chain is handled by separate actors
  ;;[1 1 1] Inteface callback from actors taking part in the event chain to inform that chain compoent is completed and the next event section will be called.
  (Variables|Default|SetCurrentEventSectionFinished? true)
  (CallFunction|NextDialogueSection))

(fn ConstructionScript)