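; Level director for a divided-room experiment trial, placing the player on the left or right per the game instance.
; A sequential MultiGate steps through word-list power-off with a distractor-task audio intro, word-list power-on, then level end.
; Separate actors run each section's content and report completion through EventSectionEnd to request the next.
; Level end fades the camera, advances the game instance's trial and opens the next level.
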(event Custom|Level%20End
  (bind _gi (Variables|Default|GetGI))
  (Default|FadeOut (Variables|Default|GetCameraFade))
  (Default|NextTrial _gi)
  (Variables|/Game/GameMode/GI_MemSeg_03.GI_MemSeg_03_C|SetTitleLvlState _gi 1)
  (Utilities|FlowControl|Delay 3.0)
  (Game|OpenLevel(byName) (Variables|Default|GetNextLevelName)))

(event Custom|Next%20Event%20Section
  ;[1 1 1] Event sequence chain logic. content for each step in the chain is handled by separate actors
  (if (Variables|Default|GetCurrentEventSectionFinished?)
    (Variables|Default|SetCurrentEventSectionFinished? false)
    (Utilities|FlowControl|MultiGate false false -1
      (:Out%200
        (bind _outactors (Actor|GetAllActorsOfClass "/Game/UI/3D_UI/BP_3DUI_AppearOnView_WordList.BP_3DUI_AppearOnView_WordList_C"))
        (for _array_element _outactors
          (Default|PowerOFF _array_element)
          (Utilities|FlowControl|Delay 5.0)
          (Class|BPIAudioComms|AudioComms(Message) (Variables|Default|GetAudioAssetsBP)) ; Introduction to distractor task
        ))
      (:Out%201
        (bind _outactors_2 (Actor|GetAllActorsOfClass "/Game/UI/3D_UI/BP_3DUI_AppearOnView_WordList.BP_3DUI_AppearOnView_WordList_C"))
        (for _array_element_2 _outactors_2
          (Default|PowerON _array_element_2)))
      (:Out%202
        (Utilities|FlowControl|Delay 3.0)
        (CallFunction|LevelEnd)))))

(event EventBeginPlay
  (Input|EnableInput (Game|GetPlayerController 0))
  (bind _asgi_mem_seg_03 (Utilities|Casting|CastToGI_MemSeg_03 (Game|GetGameInstance)))
  (Variables|Default|SetGI _asgi_mem_seg_03)
  (bind _outactors (Actor|GetAllActorsOfClass "/Game/Blueprints/Environment/BP_CameraFade.BP_CameraFade_C"))
  (Variables|Default|SetCameraFade (Utilities|Array|Get(acopy) _outactors))
  (bind _outactors_2 (Actor|GetAllActorsOfClass "/Game/Blueprints/Environment/BP_Diag_TrialRoom.BP_Diag_TrialRoom_C"))
  (Variables|Default|SetAudioAssetsBP (Utilities|Array|Get(acopy) _outactors_2))
  (if (Variables|/Game/GameMode/GI_MemSeg_03.GI_MemSeg_03_C|GetPlayerOnLeft? (Variables|Default|GetGI))
    (Transformation|SetActorLocation (Game|Player|GetPlayerPawn 0) (Variables|Default|GetPlayerLocationLeft) false true)
    (else
      (Transformation|SetActorLocation (Game|Player|GetPlayerPawn 0) (Variables|Default|GetPlayerLocationRight) false true)
      (CallFunction|NextEventSection))))

(event EventEventSectionEnd
  ;[1 1 1] Event sequence chain logic. content for each step in the chain is handled by separate actors
  ;;[1 1 1] Inteface callback from actors taking part in the event chain to inform that chain compoent is completed and the next event section will be called.
  (Development|PrintString "event fired")
  (Variables|Default|SetCurrentEventSectionFinished? true)
  (CallFunction|NextEventSection))

(fn ConstructionScript)