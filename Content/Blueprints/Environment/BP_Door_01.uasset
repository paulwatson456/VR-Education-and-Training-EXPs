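; Door Blueprint that plays close and open sounds as overlaps begin and end on its lock collision volume.
; Begin overlap plays the close cue and end overlap plays the open cue, each started at an offset.
; Volume and pitch of each cue scale with the door component's Y-axis speed, clamped separately, so the sound follows how fast the door moves.
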(event OnComponentBeginOverlap(Lock_COL)
  (params (OverlappedComponent :type Primitive%20Component%20Object%20Reference) (OtherActor :type Actor%20Object%20Reference) (OtherComp :type Primitive%20Component%20Object%20Reference) (OtherBodyIndex :type Integer) (bFromSweep :type Boolean) (SweepResult :type Hit%20Result%20Structure%20%28by%20ref%29))
  (bind _door (Variables|Default|GetDoor))
  (bind _s_freesound_doorclose_01_cue1 (Variables|Default|GetS_Freesound_DoorClose_01_Cue1))
  (bind _returnvalue (Transformation|GetComponentVelocity _door))
  (bind (_x _y) (Math|Vector|BreakVector _returnvalue))
  (bind _returnvalue_2 (Math|Conversions|ToVector(Float) _y))
  (bind _returnvalue_3 (Math|Vector|VectorLength _returnvalue_2))
  (Audio|Components|Audio|SetVolumeMultiplier _s_freesound_doorclose_01_cue1 (Math|Float|Clamp(Float) _returnvalue_3) :!class /Script/Engine.AudioComponent)
  (Audio|Components|Audio|SetPitchMultiplier _s_freesound_doorclose_01_cue1 (Math|Float|Clamp(Float) _returnvalue_3 0.0 7.0))
  (Audio|Components|Audio|Play _s_freesound_doorclose_01_cue1 0.5))

(event OnComponentEndOverlap(Lock_COL)
  (params (OverlappedComponent :type Primitive%20Component%20Object%20Reference) (OtherActor :type Actor%20Object%20Reference) (OtherComp :type Primitive%20Component%20Object%20Reference) (OtherBodyIndex :type Integer))
  (bind _door (Variables|Default|GetDoor))
  (bind _s_freesound_dooropen_02_cue (Variables|Default|GetS_Freesound_DoorOpen_02_Cue))
  (bind _returnvalue (Transformation|GetComponentVelocity _door))
  (bind (_x _y) (Math|Vector|BreakVector _returnvalue))
  (bind _returnvalue_2 (Math|Conversions|ToVector(Float) _y))
  (bind _returnvalue_3 (Math|Vector|VectorLength _returnvalue_2))
  (Audio|Components|Audio|SetVolumeMultiplier _s_freesound_dooropen_02_cue (Math|Float|Clamp(Float) _returnvalue_3) :!class /Script/Engine.AudioComponent)
  (Audio|Components|Audio|SetPitchMultiplier _s_freesound_dooropen_02_cue (Math|Float|Clamp(Float) _returnvalue_3 0.0 7.0))
  (Audio|Components|Audio|Play _s_freesound_dooropen_02_cue 0.5))

(fn ConstructionScript)