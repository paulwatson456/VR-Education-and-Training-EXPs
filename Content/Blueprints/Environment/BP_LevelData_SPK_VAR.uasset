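; Level data Blueprint that loads one row of counterbalanced trial factors from the MemSeg_03 data table into a map.
; On BeginPlay it reads the hardcoded row P02 and fetches the table's "RowNames" column as strings.
; NewFunction0 splits that list by index into map keys, paired in fixed order with the row's trial fields, some converted to strings.
; The result is stored in TableDataMap.
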(event EventBeginPlay
  (bind _returnvalue (Utilities|GetDataTableRow "/Game/DataTables/MemSeg_03_CounterbalancedFactors_01.MemSeg_03_CounterbalancedFactors_01" "P02")
    (:then
      (bind _returnvalue_2 (Class|DataTableFunctionLibrary|GetDataTableColumnasString "/Game/DataTables/MemSeg_03_CounterbalancedFactors_01.MemSeg_03_CounterbalancedFactors_01" "RowNames"))
      (bind (_columnname01 _columnname02 _columnname03 _columnname04 _columnname05 _columnname06 _columnname07 _columnname08 _columnname09 _columnname10 _columnname11 _columnname12 _columnname13 _columnname14 _columnname15 _columnname16 _columnname17 _columnname18 _columnname19 _columnname20 _columnname21 _columnname22 _columnname23 _columnname24 _columnname25 _columnname26 _columnname27 _columnname28 _columnname29 _columnname30 _columnname31 _columnname32 _columnname33 _columnname34 _columnname35 _columnname36) (CallFunction|NewFunction0 _returnvalue_2))
      (Variables|Default|SetTableDataMap (Utilities|Map|MakeMap _columnname01 (.TR_01 (Utilities|Struct|BreakMemSeg_03_CounterbalancedFactors _returnvalue)) _columnname02 (.TR_02 (Utilities|Struct|BreakMemSeg_03_CounterbalancedFactors _returnvalue)) _columnname03 (.TR_03 (Utilities|Struct|BreakMemSeg_03_CounterbalancedFactors _returnvalue)) _columnname04 (.TR_04 (Utilities|Struct|BreakMemSeg_03_CounterbalancedFactors _returnvalue)) _columnname05 (.TR_01_RM (Utilities|Struct|BreakMemSeg_03_CounterbalancedFactors _returnvalue)) _columnname06 (.TR_02_RM (Utilities|Struct|BreakMemSeg_03_CounterbalancedFactors _returnvalue)) _columnname07 (.TR_03_RM (Utilities|Struct|BreakMemSeg_03_CounterbalancedFactors _returnvalue)) _columnname08 (.TR_04_RM (Utilities|Struct|BreakMemSeg_03_CounterbalancedFactors _returnvalue)) _columnname09 (Utilities|String|ToString(Integer) (.TR_01_WL_SP1 (Utilities|Struct|BreakMemSeg_03_CounterbalancedFactors _returnvalue))) _columnname10 (Utilities|String|ToString(Integer) (.TR_01_WL_SP2 (Utilities|Struct|BreakMemSeg_03_CounterbalancedFactors _returnvalue))) _columnname11 (Utilities|String|ToString(Integer) (.TR_02_WL_SP1 (Utilities|Struct|BreakMemSeg_03_CounterbalancedFactors _returnvalue))) _columnname12 (Utilities|String|ToString(Integer) (.TR_02_WL_SP2 (Utilities|Struct|BreakMemSeg_03_CounterbalancedFactors _returnvalue))) _columnname13 (Utilities|String|ToString(Integer) (.TR_03_WL_SP1 (Utilities|Struct|BreakMemSeg_03_CounterbalancedFactors _returnvalue))) _columnname14 (Utilities|String|ToString(Integer) (.TR_03_WL_SP2 (Utilities|Struct|BreakMemSeg_03_CounterbalancedFactors _returnvalue))) _columnname15 (Utilities|String|ToString(Integer) (.TR_04_WL_SP1 (Utilities|Struct|BreakMemSeg_03_CounterbalancedFactors _returnvalue))) _columnname16 (Utilities|String|ToString(Integer) (.TR_04_WL_SP2 (Utilities|Struct|BreakMemSeg_03_CounterbalancedFactors _returnvalue))) _columnname17 (.TR_01_V_SP1 (Utilities|Struct|BreakMemSeg_03_CounterbalancedFactors _returnvalue)) _columnname18 (.TR_01_V_SP2 (Utilities|Struct|BreakMemSeg_03_CounterbalancedFactors _returnvalue)) _columnname19 (.TR_02_V_SP1 (Utilities|Struct|BreakMemSeg_03_CounterbalancedFactors _returnvalue)) _columnname20 (.TR_02_V_SP2 (Utilities|Struct|BreakMemSeg_03_CounterbalancedFactors _returnvalue)) _columnname21 (.TR_03_V_SP1 (Utilities|Struct|BreakMemSeg_03_CounterbalancedFactors _returnvalue)) _columnname22 (.TR_03_V_SP2 (Utilities|Struct|BreakMemSeg_03_CounterbalancedFactors _returnvalue)) _columnname23 (.TR_04_V_SP1 (Utilities|Struct|BreakMemSeg_03_CounterbalancedFactors _returnvalue)) _columnname24 (.TR_04_V_SP2 (Utilities|Struct|BreakMemSeg_03_CounterbalancedFactors _returnvalue)) _columnname25 (Utilities|String|ToString(Integer) (.TR_01_SP_SP1 (Utilities|Struct|BreakMemSeg_03_CounterbalancedFactors _returnvalue))) _columnname26 (Utilities|String|ToString(Integer) (.TR_01_SP_SP2 (Utilities|Struct|BreakMemSeg_03_CounterbalancedFactors _returnvalue))) _columnname27 (Utilities|String|ToString(Integer) (.TR_02_SP_SP1 (Utilities|Struct|BreakMemSeg_03_CounterbalancedFactors _returnvalue))) _columnname28 (Utilities|String|ToString(Integer) (.TR_02_SP_SP2 (Utilities|Struct|BreakMemSeg_03_CounterbalancedFactors _returnvalue))) _columnname29 (Utilities|String|ToString(Integer) (.TR_03_SP_SP1 (Utilities|Struct|BreakMemSeg_03_CounterbalancedFactors _returnvalue))) _columnname30 (Utilities|String|ToString(Integer) (.TR_03_SP_SP2 (Utilities|Struct|BreakMemSeg_03_CounterbalancedFactors _returnvalue))) _columnname31 (Utilities|String|ToString(Integer) (.TR_04_SP_SP1 (Utilities|Struct|BreakMemSeg_03_CounterbalancedFactors _returnvalue))) _columnname32 (Utilities|String|ToString(Integer) (.TR_04_SP_SP2 (Utilities|Struct|BreakMemSeg_03_CounterbalancedFactors _returnvalue))) _columnname33 (Utilities|String|ToString(Integer) (.TR_01_StartPos (Utilities|Struct|BreakMemSeg_03_CounterbalancedFactors _returnvalue))) _columnname34 (Utilities|String|ToString(Integer) (.TR_02_StartPos (Utilities|Struct|BreakMemSeg_03_CounterbalancedFactors _returnvalue))) _columnname35 (Utilities|String|ToString(Integer) (.TR_03_StartPos (Utilities|Struct|BreakMemSeg_03_CounterbalancedFactors _returnvalue))) _columnname36 (Utilities|String|ToString(Integer) (.TR_04_StartPos (Utilities|Struct|BreakMemSeg_03_CounterbalancedFactors _returnvalue))))))))

(fn ConstructionScript)

(fn NewFunction0
  (params (ListOfColumnNames :type Array%20of%20Strings))
  (return (Utilities|Array|Get(acopy) ListOfColumnNames) (Utilities|Array|Get(acopy) ListOfColumnNames 1) (Utilities|Array|Get(acopy) ListOfColumnNames 2) (Utilities|Array|Get(acopy) ListOfColumnNames 3) (Utilities|Array|Get(acopy) ListOfColumnNames 4) (Utilities|Array|Get(acopy) ListOfColumnNames 5) (Utilities|Array|Get(acopy) ListOfColumnNames 6) (Utilities|Array|Get(acopy) ListOfColumnNames 7) (Utilities|Array|Get(acopy) ListOfColumnNames 8) (Utilities|Array|Get(acopy) ListOfColumnNames 9) (Utilities|Array|Get(acopy) ListOfColumnNames 10) (Utilities|Array|Get(acopy) ListOfColumnNames 11) (Utilities|Array|Get(acopy) ListOfColumnNames 12) (Utilities|Array|Get(acopy) ListOfColumnNames 13) (Utilities|Array|Get(acopy) ListOfColumnNames 14) (Utilities|Array|Get(acopy) ListOfColumnNames 15) (Utilities|Array|Get(acopy) ListOfColumnNames 16) (Utilities|Array|Get(acopy) ListOfColumnNames 17) (Utilities|Array|Get(acopy) ListOfColumnNames 18) (Utilities|Array|Get(acopy) ListOfColumnNames 19) (Utilities|Array|Get(acopy) ListOfColumnNames 20) (Utilities|Array|Get(acopy) ListOfColumnNames 21) (Utilities|Array|Get(acopy) ListOfColumnNames 22) (Utilities|Array|Get(acopy) ListOfColumnNames 23) (Utilities|Array|Get(acopy) ListOfColumnNames 24) (Utilities|Array|Get(acopy) ListOfColumnNames 25) (Utilities|Array|Get(acopy) ListOfColumnNames 26) (Utilities|Array|Get(acopy) ListOfColumnNames 27) (Utilities|Array|Get(acopy) ListOfColumnNames 28) (Utilities|Array|Get(acopy) ListOfColumnNames 29) (Utilities|Array|Get(acopy) ListOfColumnNames 30) (Utilities|Array|Get(acopy) ListOfColumnNames 31) (Utilities|Array|Get(acopy) ListOfColumnNames 32) (Utilities|Array|Get(acopy) ListOfColumnNames 33) (Utilities|Array|Get(acopy) ListOfColumnNames 34) (Utilities|Array|Get(acopy) ListOfColumnNames 35)))