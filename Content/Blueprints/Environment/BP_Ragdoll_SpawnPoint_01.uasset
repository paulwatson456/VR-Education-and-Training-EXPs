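; Spawn point that places a ragdoll actor in the level and replaces it when the recovery instruction menu requests a reset.
; After a startup delay, BeginPlay binds to the ResetRagdoll dispatcher on the 3D menu's widget, then spawns the first ragdoll after another delay.
; Spawning uses a configurable offset and rotation, and each reset destroys the stored ragdoll before respawning.
; Failed menu or widget casts prevent the initial spawn.
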(event Custom|Spawn%20Ragdoll
  (bind _returnvalue (Game|SpawnActorfromClass "/Game/ContentPacks/Mannequin/Character/Mesh/RagdollBP.RagdollBP_C" (Math|Transform|MakeTransform (+ (Transformation|GetWorldLocation (Variables|Default|GetDefaultSceneRoot)) (Variables|Default|GetSpawnLocationRelative)) (Variables|Default|GetSpawnRotation)) "Undefined" 0 0))
  (Variables|Default|SetRagdollActor _returnvalue))

(event Custom|ResetRagdoll_Event_0
  (Actor|DestroyActor (Variables|Default|GetRagdollActor))
  (CallFunction|SpawnRagdoll))

(event EventBeginPlay
  (Utilities|FlowControl|Delay 3.0)
  (Variables|Default|Set3DMenu (Variables|Default|Get3DMenu))
  (bind _asui3d_ragdoll_menu_01 (Utilities|Casting|CastToUI3D_RagdollMenu_01 (Variables|Default|Get3DMenu)))
  (bind _asui_w_recovery_instruction (Utilities|Casting|CastToUI_W_RecoveryInstruction (UserInterface|GetWidget (Variables|/Game/UI/3D_UI/UI3D_RagdollMenu_01.UI3D_RagdollMenu_01_C|GetMenu _asui3d_ragdoll_menu_01))))
  (EventDispatchers|AssignResetRagdoll _asui_w_recovery_instruction (delegate Custom|ResetRagdoll_Event_0))
  (Utilities|FlowControl|Delay 1.0)
  (bind _returnvalue (Game|SpawnActorfromClass "/Game/ContentPacks/Mannequin/Character/Mesh/RagdollBP.RagdollBP_C" (Math|Transform|MakeTransform (+ (Transformation|GetWorldLocation (Variables|Default|GetDefaultSceneRoot)) (Variables|Default|GetSpawnLocationRelative)) (Variables|Default|GetSpawnRotation)) "Undefined" 0 0))
  (Variables|Default|SetRagdollActor _returnvalue))

(event Collision|EventActorBeginOverlap
  (params (OtherActor :type Actor%20Object%20Reference)))

(event EventTick
  (params (DeltaSeconds :type Float%20%28single-precision%29)))

(fn ConstructionScript)