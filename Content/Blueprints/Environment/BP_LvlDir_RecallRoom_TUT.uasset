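; Level director for the recall room tutorial, sequencing dialogue and a maths distractor task before moving on.
; A MultiGate steps through intro, challenge, recall instruction and closing dialogue, messaging separate dialogue and challenge actors found at BeginPlay.
; Those actors report back through an interface callback, EventSectionEnd, to trigger the next step.
; The last step fades the camera and opens either the game instance's next trial room (whole or divided) or a named level.
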(event Custom|Level%20End
  (if (Variables|Default|GetMovingToNextTrial)
    (Default|FadeOut (Variables|Default|GetCameraFade))
    (Default|NextTrial (Variables|Default|GetGI))
    (Utilities|FlowControl|Delay 3.0)
    (if (<= (Variables|/Game/GameMode/GI_MemSeg_03.GI_MemSeg_03_C|GetNextRoomNumber (Variables|Default|GetGI)) 1)
      (Game|OpenLevel(byName) "EXP_03_Room_Whole")
      (else
        (Game|OpenLevel(byName) "EXP_03_Room_Divided")))
    (else
      (Default|FadeOut (Variables|Default|GetCameraFade))
      (Utilities|FlowControl|Delay 3.0)
      (Game|OpenLevel(byName) (Variables|Default|GetNextLevelName)))))

(event Custom|Next%20Event%20Section
  ;[1 1 1] Event sequence chain logic. content for each step in the chain is handled by separate actors
  (if (Variables|Default|GetCurrentEventSectionFinished?)
    (Variables|Default|SetCurrentEventSectionFinished? false)
    (Utilities|FlowControl|MultiGate false false -1
      (:Out%200
        (Class|BPIAudioComms|AudioComms(Message) (Variables|Default|GetAudioAssetsBP)) ; Introduction to distractor task
      )
      (:Out%201
        (Class|BPIChallengeComms|ChallengeComms(Message) (Variables|Default|GetChallengeBP)) ; Activate distarctor task
      )
      (:Out%202
        (Class|BPIAudioComms|AudioComms(Message) (Variables|Default|GetAudioAssetsBP)) ; Challenge complete dialogue and recall instruction
      )
      (:Out%203
        (Class|BPIAudioComms|AudioComms(Message) (Variables|Default|GetAudioAssetsBP)) ; recall complete and next instructions
      )
      (:Out%204
        (CallFunction|LevelEnd)))))

(event EventBeginPlay
  (Input|EnableInput (Game|GetPlayerController 0))
  (bind _asgi_mem_seg_03 (Utilities|Casting|CastToGI_MemSeg_03 (Game|GetGameInstance)))
  (Variables|Default|SetGI _asgi_mem_seg_03)
  (bind _outactors (Actor|GetAllActorsOfClass "/Game/Blueprints/Environment/BP_CameraFade.BP_CameraFade_C"))
  (Variables|Default|SetCameraFade (Utilities|Array|Get(acopy) _outactors))
  (bind _outactors_2 (Actor|GetAllActorsOfClass "/Game/Blueprints/Environment/BP_Diag_RecallRoom_TUT_01.BP_Diag_RecallRoom_TUT_01_C"))
  (Variables|Default|SetAudioAssetsBP (Utilities|Array|Get(acopy) _outactors_2))
  (bind _outactors_3 (Actor|GetAllActorsOfClass "/Game/Blueprints/DistractionTask/BP_DistractionTask_Maths_02.BP_DistractionTask_Maths_02_C"))
  (Variables|Default|SetChallengeBP (Utilities|Array|Get(acopy) _outactors_3))
  (CallFunction|NextEventSection))

(event EventEventSectionEnd
  ;[1 1 1] Event sequence chain logic. content for each step in the chain is handled by separate actors
  ;;[1 1 1] Inteface callback from actors taking part in the event chain to inform that chain compoent is completed and the next event section will be called.
  (Variables|Default|SetCurrentEventSectionFinished? true)
  (CallFunction|NextEventSection))

(fn ConstructionScript)