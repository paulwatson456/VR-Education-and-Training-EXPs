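; BP_PowerManager_01 is a trigger-box power switch that sends power on and off messages to a referenced SubjectToPower01.
; Any begin or end overlap on the box sends the matching message, plays a sound and updates PowerIsOn.
; One second after BeginPlay it sends power off, then box-traces at the box and restores power for hit components tagged PlayerBody, without setting PowerIsOn.
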(event OnComponentBeginOverlap(Box)
  (params (OverlappedComponent :type Primitive%20Component%20Object%20Reference) (OtherActor :type Actor%20Object%20Reference) (OtherComp :type Primitive%20Component%20Object%20Reference) (OtherBodyIndex :type Integer) (bFromSweep :type Boolean) (SweepResult :type Hit%20Result%20Structure%20%28by%20ref%29))
  (Utilities|IsValid (Variables|Default|GetSubjectToPower_01)
    (:Is%20Valid
      (Class|BPIPowerON|PowerON(Message) (Variables|Default|GetSubjectToPower_01)))
    (:Is%20Not%20Valid
      _))
  (Audio|PlaySoundatLocation "/Game/Sound/UI/S_PowerOn_01.S_PowerOn_01" (Transformation|GetWorldLocation (Variables|Default|GetBox)) "0, 0, 0" 0.1 1.0 0.0 0 0 0)
  (Variables|Default|SetPowerIsOn? true))

(event OnComponentEndOverlap(Box)
  (params (OverlappedComponent :type Primitive%20Component%20Object%20Reference) (OtherActor :type Actor%20Object%20Reference) (OtherComp :type Primitive%20Component%20Object%20Reference) (OtherBodyIndex :type Integer))
  (Utilities|IsValid (Variables|Default|GetSubjectToPower_01)
    (:Is%20Valid
      (Class|BPIPowerOFF|PowerOFF(Message) (Variables|Default|GetSubjectToPower_01)))
    (:Is%20Not%20Valid
      _))
  (Audio|PlaySoundatLocation "/Game/Sound/UI/S_PowerOff_01.S_PowerOff_01" (Transformation|GetWorldLocation (Variables|Default|GetBox)) "0, 0, 0" 0.1 1.0 0.0 0 0 0)
  (Variables|Default|SetPowerIsOn? false))

(event EventBeginPlay
  (bind _box (Variables|Default|GetBox))
  (bind _returnvalue (Transformation|GetWorldLocation _box))
  (Utilities|FlowControl|Delay 1.0)
  (Class|BPIPowerOFF|PowerOFF(Message) (Variables|Default|GetSubjectToPower_01))
  (bind _outhits (Class|KismetSystemLibrary|BoxTraceMulti _returnvalue _returnvalue "25.000000,25.000000,30.000000" "0, 0, 0" "TraceTypeQuery1" false 0 "None" true))
  (for _array_element _outhits
    (if (Components|ComponentHasTag (.hitcomponent _array_element) "PlayerBody")
      (Class|BPIPowerON|PowerON(Message) (Variables|Default|GetSubjectToPower_01)))))

(fn ConstructionScript)