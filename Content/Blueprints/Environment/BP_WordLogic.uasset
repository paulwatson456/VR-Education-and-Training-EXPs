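; Speaker actor that plays a randomized spoken word list at its location for a trial, with an optional in-world info widget.
; AddLevelData shuffles and trims the item indices to the list size, saving the order for identical replays.
; ActivateCommand starts a delayed recursive loop that plays items from the array's end, with word list IDs 9–16 reusing lists 1–8.
; After the final allowed play-through, it notifies the speaker manager.
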(event Custom|AddLevelData
  (bind _infopointitemnum (Variables|Default|GetInfoPointItemNum))
  (if (Variables|Default|GetUsesDataTable)
    (Utilities|FlowControl|Delay 0.1)
    (Variables|/Game/UI/3D_UI/UI_W_DataTableVis.UI_W_DataTableVis_C|SetListLength (Variables|Default|GetSpeakerInfo) (Variables|Default|GetList%20size))
    (Variables|/Game/UI/3D_UI/UI_W_DataTableVis.UI_W_DataTableVis_C|SetSpeakerNumber (Variables|Default|GetSpeakerInfo) (Variables|Default|GetSpeakerID))
    (Variables|/Game/UI/3D_UI/UI_W_DataTableVis.UI_W_DataTableVis_C|SetTrialLetter (Variables|Default|GetSpeakerInfo) (Variables|Default|GetTrialCondition))
    (Variables|/Game/UI/3D_UI/UI_W_DataTableVis.UI_W_DataTableVis_C|SetWordListNumber (Variables|Default|GetSpeakerInfo) (Variables|Default|GetWordListID)))
  (Input|EnableInput (Game|GetPlayerController 0))
  ;[1 1 1] Creates a 10 item array, randomises the order and resizes to required number of elements for trial
  (Utilities|Array|Shuffle (Variables|Default|GetInfoPointItemNum))
  (Utilities|Array|Resize _infopointitemnum (Variables|Default|GetList%20size))
  (Variables|Default|SetInfoPointItemNumSave _infopointitemnum))

(event Custom|PlayThroughInformation
  (if (== (Variables|Default|GetList%20size) (Variables|Default|GetNumInfoDelivered))
    (Audio|PlaySoundatLocation "/Game/Sound/Environment/S_Confim_01.S_Confim_01" (Transformation|GetWorldLocation (Variables|Default|GetDefaultSceneRoot self)) "0, 0, 0" 1.0 1.0 0.0 0 0 0)
    (Utilities|FlowControl|Delay 1.0)
    (Variables|Default|SetIsPlaying? false)
    (Variables|Default|SetInfoPointItemNum (Variables|Default|GetInfoPointItemNumSave))
    (Variables|Default|SetNumInfoDelivered 0)
    (if (== (Variables|Default|GetNumPlayThroughs) (Variables|Default|GetMaxNumPlayThroughs))
      (Default|DeliveredInfoPointEvent (Variables|Default|GetSpeakerManager)))
    (else
      ;[1 1 1] Delivers information point at last position in array
      (bind _output_get (Variables|Default|SetInfoItemToBeDelivered (Utilities|Array|Get(acopy) (Variables|Default|GetInfoPointItemNum) (Utilities|Array|LastIndex (Variables|Default|GetInfoPointItemNum)))))
      (Development|PrintString (Utilities|String|ToString(Integer) _output_get))
      (switch int (Variables|Default|GetWordListID)
        (:1
          (CallFunction|DeliverInfo (Variables|Default|GetWordList_01) :!label _label))
        (:2
          (CallFunction|DeliverInfo (Variables|Default|GetWordList_02) :!label _label_2))
        (:3
          (CallFunction|DeliverInfo (Variables|Default|GetWordList_03) :!label _label_3))
        (:4
          (CallFunction|DeliverInfo (Variables|Default|GetWordList_04) :!label _label_4))
        (:5
          (CallFunction|DeliverInfo (Variables|Default|GetWordList_05) :!label _label_5))
        (:6
          (CallFunction|DeliverInfo (Variables|Default|GetWordList_06) :!label _label_6))
        (:7
          (CallFunction|DeliverInfo (Variables|Default|GetWordList_07) :!label _label_7))
        (:8
          (CallFunction|DeliverInfo (Variables|Default|GetWordList_08) :!label _label_8))
        (:9
          (goto _label))
        (:10
          (goto _label_2))
        (:11
          (goto _label_3))
        (:12
          (goto _label_4))
        (:13
          (goto _label_5))
        (:14
          (goto _label_6))
        (:15
          (goto _label_7))
        (:16
          (goto _label_8)))
      ;[1 1 1] Removes last position point in array, reducing the size each run through
      (Utilities|Array|RemoveIndex (Variables|Default|GetInfoPointItemNum) (Utilities|Array|LastIndex (Variables|Default|GetInfoPointItemNum)))
      (Utilities|FlowControl|Delay (+ (Variables|Default|GetInfoDuration) 1.0))
      (Variables|Default|SetNumInfoDelivered (+ (Variables|Default|GetNumInfoDelivered) 1))
      (CallFunction|PlayThroughInformation))))

(event EventBeginPlay
  (bind _datatable_vis (Variables|Default|GetDataTable_Vis))
  (bind _outactors (Actor|GetAllActorsOfClass "/Game/Blueprints/Environment/BP_SpeakerManager_Base.BP_SpeakerManager_Base_C"))
  (Variables|Default|SetSpeakerManager (Utilities|Array|Get(acopy) _outactors))
  (if (Variables|Default|GetCanViewSpeakerInfo?)
    (bind _asui_w_data_table_vis (Utilities|Casting|CastToUI_W_DataTableVis (UserInterface|GetUserWidgetObject (Variables|Default|GetDataTable_Vis))))
    (Variables|Default|SetSpeakerInfo _asui_w_data_table_vis)
    (else
      (Rendering|SetVisibility _datatable_vis false false)
      (Collision|SetCollisionEnabled _datatable_vis "NoCollision"))))

(event EventActivateCommand
  (if (not (== (Variables|Default|GetNumPlayThroughs) (Variables|Default|GetMaxNumPlayThroughs)))
    (if (not (Variables|Default|GetIsPlaying?))
      (Variables|Default|SetIsPlaying? true)
      (Audio|PlaySoundatLocation "/Game/Sound/Environment/S_Confim_01.S_Confim_01" "0, 0, 0" "0, 0, 0" 1.0 1.0 0.0 0 0 0)
      (Utilities|FlowControl|Delay 1.0)
      (Variables|Default|SetNumPlayThroughs (+ (Variables|Default|GetNumPlayThroughs) 1))
      (CallFunction|PlayThroughInformation))))

(event Input|KeyboardEvents|9
  (params (Key :type Key%20Structure :default "None"))
  (:Pressed
    (Development|PrintString (Utilities|String|ToString(Integer) (Utilities|Array|Length (Variables|Default|GetInfoPointItemNum))))))

(fn ConstructionScript)

(fn DeliverInfo
  (params (InformationList :type Array%20of%20Sound%20Base%20Object%20References))
  (bind _infoitemtobedelivered (Variables|Default|GetInfoItemToBeDelivered))
  (bind _output (Utilities|Array|Get(acopy) InformationList _infoitemtobedelivered))
  (Audio|PlaySoundatLocation _output (Transformation|GetWorldLocation (Variables|Default|GetDefaultSceneRoot self)) "0, 0, 0" 2.0 1.0 0.0 "/Game/Sound/Attenuation/Attenuation_01.Attenuation_01" 0 0)
  (Variables|Default|SetInfoDuration (Variables|/Script/Engine.SoundBase|GetDuration _output)))