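; Level director for the SPK VAR title level, running either a tutorial or a trial sequence based on LevelType.
; On BeginPlay it spawns a power manager and floor icon for both start types.
; Each NextEventSection call advances a MultiGate through narration (tutorial only), UI spawning and level end.
; Spawned UI registers with the power manager, showing a power-off message when unpowered; player-facing placement logic is left unwired.
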(event Custom|Start%20Tutorial
  (Utilities|FlowControl|MultiGate false false -1
    (:Out%200
      (Utilities|FlowControl|Delay 4.0)
      (Class|INTLevelCommands|LevelEventPlayAudio(Message) (Variables|Default|GetAudioNarrationBP_01)))
    (:Out%201
      (CallFunction|SpawnNextUI)
      (bind _asbp_keypad (Utilities|Casting|CastToBP_Keypad (Variables|Default|GetCurrentUI)))
      (Variables|/Game/UI/3D_UI/BP_Keypad.BP_Keypad_C|SetLevelDirectorREF _asbp_keypad self))
    (:Out%202
      (CallFunction|LevelEndSPKVAR))))

(event Custom|DestroyUI
  (Actor|DestroyActor (Variables|Default|GetCurrentUI))
  (Variables|Default|SetUI_To_Spawn (+ (Variables|Default|GetUI_To_Spawn) 1)))

(event Custom|Spawn%20Next%20UI
  (bind _returnvalue (Game|SpawnActorfromClass (Utilities|Array|Get(acopy) (Variables|Default|GetUI_ActorsToSpawn) (Variables|Default|GetUI_To_Spawn)) (Math|Transform|MakeTransform "0, 0, 0") "Undefined" 0 0))
  (bind _output_get (Variables|Default|SetCurrentUI _returnvalue))
  (CallFunction|AssignCurrentUItoPowerManager))

(event Custom|Start%20Trial
  (Utilities|FlowControl|MultiGate false false -1
    (:Out%200
      (Variables|Default|SetUI_To_Spawn 1)
      (CallFunction|SpawnNextUI))
    (:Out%201
      (CallFunction|LevelEndSPKVAR))))

(event EventBeginPlay
  (|CallParentFunction)
  (switch Utilities|FlowControl|Switch|SwitchonEN_Tile_LevelType_01 (Utilities|Enum|ByteToEnumEN_Tile_LevelType_01 (Variables|Default|GetLevelType))
    (:NewEnumerator0
      _)
    (:NewEnumerator2
      _))
  (bind _returnvalue (Game|SpawnActorfromClass "/Game/Blueprints/Environment/BP_PowerManager_01.BP_PowerManager_01_C" (Math|Transform|MakeTransform "20.000000,30.000000,-110.000000" "0.000000,180.000000,0.000000") "Undefined" 0 0))
  (Variables|Default|SetPowerREF _returnvalue)
  (Game|SpawnActorfromClass "/Game/UI/3D_UI/3DUI_FloorIcon_01.3DUI_FloorIcon_01_C" (Math|Transform|MakeTransform "20.000000,30.000000,-110.000000" "0.000000,180.000000,0.000000") "Undefined" 0 0))

(event EventNextEventSection
  (CallFunction|NextEventCheck)
  (switch Utilities|FlowControl|Switch|SwitchonEN_Tile_LevelType_01 (Utilities|Enum|ByteToEnumEN_Tile_LevelType_01 (Variables|Default|GetLevelType))
    (:NewEnumerator0
      (CallFunction|StartTutorial)
      (Variables|Default|SetMovingToNextTrial false))
    (:NewEnumerator2
      (CallFunction|StartTrial)
      (Variables|Default|SetMovingToNextTrial true))))

(fn ConstructionScript
  (|CallParentFunction))

(fn UIPosition+Height
  (return (Math|Conversions|ToTransform(Vector) (* (Transformation|GetActorForwardVector (Game|Player|GetPlayerPawn 0)) 1e+02))))

(fn AssignCurrentUItoPowerManager
  (bind _asbp_power_manager_01 (Utilities|Casting|CastToBP_PowerManager_01 (Variables|Default|GetPowerREF)))
  (bind _output_get (Variables|/Game/Blueprints/Environment/BP_PowerManager_01.BP_PowerManager_01_C|SetSubjectToPower_01 _asbp_power_manager_01 (Variables|Default|GetCurrentUI)))
  (Utilities|IsValid _output_get
    (:Is%20Valid
      (bind _asbp_power_manager_01_2 (Utilities|Casting|CastToBP_PowerManager_01 (Variables|Default|GetPowerREF)))
      (if (not (Variables|/Game/Blueprints/Environment/BP_PowerManager_01.BP_PowerManager_01_C|GetPowerIsOn? _asbp_power_manager_01_2))
        (Class|BPIPowerOFF|PowerOFF(Message) (Variables|Default|GetCurrentUI))))))

(fn SetUIRotationTowardsPlayer
  (params (UI_ActorToRotate :type Actor%20Object%20Reference))
  (bind _returnvalue (Game|Player|GetPlayerPawn 0))
  (bind _returnvalue_2 (Transformation|GetActorForwardVector _returnvalue))
  (bind _returnvalue_3 (Math|Conversions|RotationFromXVector _returnvalue_2))
  (Transformation|SetActorRotation UI_ActorToRotate (Math|Rotator|MakeRotator (.roll _returnvalue_3) (.pitch _returnvalue_3) (- (.yaw _returnvalue_3) 1.8e+02))))