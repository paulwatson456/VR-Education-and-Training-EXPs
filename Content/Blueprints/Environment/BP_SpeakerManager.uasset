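; BP_SpeakerManager configures two speaker actors, SPA and SPB, for a trial when the level begins.
; It reads the first BP_GatherLevelAttributes actor, giving each speaker its own ID and word list but a shared list size and trial condition.
; After pushing these values, it calls AddLevelData on both speakers.
; It also counts delivered info point events, though reaching two triggers nothing yet.
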(event Custom|DeliveredInfoPoint_Event
  (bind _output_get (Variables|Default|SetNumbDeliveredInfoPoints (+ (Variables|Default|GetNumbDeliveredInfoPoints) 1)))
  (if (>= _output_get 2)
    _))

(event EventBeginPlay
  (EventDispatchers|BindEventtoDeliveredInfoPoint (delegate Custom|DeliveredInfoPoint_Event))
  (bind _outactors (Actor|GetAllActorsOfClass "/Game/Blueprints/Environment/BP_GatherLevelAttributes.BP_GatherLevelAttributes_C"))
  (bind _output_get (Variables|Default|SetSpeakerData _outactors))
  (CallFunction|GetSpeakerData _output_get)
  (CallFunction|SetSpeakerData (Variables|Default|GetSPA) (Variables|Default|GetSPA_ListSize) (Variables|Default|GetSPA_WordList_ID) (Variables|Default|GetSPA_ID) (Variables|Default|GetSPA_TrialCondition))
  (CallFunction|SetSpeakerData (Variables|Default|GetSPB) (Variables|Default|GetSPB_ListSize) (Variables|Default|GetSPB_WordList_ID) (Variables|Default|GetSPB_ID) (Variables|Default|GetSPB_TrialCondition))
  (Default|AddLevelData (Variables|Default|GetSPA))
  (Default|AddLevelData (Variables|Default|GetSPB)))

(fn ConstructionScript)

(fn SetSpeakerData
  (params (Speaker :type BP%20Word%20Logic%20Object%20Reference) (ListSize :type Integer) (WordListNumber :type Integer) (SpeakerID :type String) (TrialCondition :type String))
  (Variables|/Game/Blueprints/Environment/BP_WordLogic.BP_WordLogic_C|SetList%20size Speaker ListSize)
  (Variables|/Game/Blueprints/Environment/BP_WordLogic.BP_WordLogic_C|SetWordListID Speaker WordListNumber)
  (Variables|/Game/Blueprints/Environment/BP_WordLogic.BP_WordLogic_C|SetSpeakerID Speaker SpeakerID)
  (Variables|/Game/Blueprints/Environment/BP_WordLogic.BP_WordLogic_C|SetTrialCondition Speaker TrialCondition))

(fn GetSpeakerData
  (params (NewParam :type Array%20of%20BP%20Gather%20Level%20Attributes%20Object%20References))
  (bind _output (Utilities|Array|Get(acopy) NewParam))
  (bind _list_size (Variables|/Game/Blueprints/Environment/BP_GatherLevelAttributes.BP_GatherLevelAttributes_C|GetList%20size _output))
  (bind _trialcondition (Variables|/Game/Blueprints/Environment/BP_GatherLevelAttributes.BP_GatherLevelAttributes_C|GetTrialCondition _output))
  (Variables|Default|SetSPA_ListSize _list_size)
  (Variables|Default|SetSPB_ListSize _list_size)
  (Variables|Default|SetSPA_WordList_ID (Variables|/Game/Blueprints/Environment/BP_GatherLevelAttributes.BP_GatherLevelAttributes_C|GetWordListNumberSPA _output))
  (Variables|Default|SetSPB_WordList_ID (Variables|/Game/Blueprints/Environment/BP_GatherLevelAttributes.BP_GatherLevelAttributes_C|GetWordListNumberSPB _output))
  (Variables|Default|SetSPA_ID (Variables|/Game/Blueprints/Environment/BP_GatherLevelAttributes.BP_GatherLevelAttributes_C|GetSPA_ID _output))
  (Variables|Default|SetSPB_ID (Variables|/Game/Blueprints/Environment/BP_GatherLevelAttributes.BP_GatherLevelAttributes_C|GetSPB_ID _output))
  (Variables|Default|SetSPA_TrialCondition _trialcondition)
  (Variables|Default|SetSPB_TrialCondition _trialcondition))