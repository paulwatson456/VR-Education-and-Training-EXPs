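; Base speaker Blueprint that plays a randomised word list as positional audio for a trial, with a selectable speaker mesh.
; On BeginPlay it shuffles and trims the index array to the list size, saves it, then applies the mesh.
; PressButton starts a limited playthrough that recursively plays and pops the last index, waiting each sound's duration.
; Each pass restores the saved order; after the final one it notifies the BP_Speaker_Gameplay_Base manager.
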(event Custom|PlayThroughInformation
  (if (== (Variables|Default|GetList%20size) (Variables|Default|GetNumWordsDelivered))
    (Audio|PlaySoundatLocation "/Game/Sound/Environment/S_Confim_01.S_Confim_01" (Transformation|GetWorldLocation (Variables|Default|GetDefaultSceneRoot)) "0, 0, 0" 1.0 1.0 0.0 0 0 0)
    (Utilities|FlowControl|Delay 1.0)
    (Variables|Default|SetIsPlaying? false)
    (Variables|Default|SetInfoPointItemNum (Variables|Default|GetInfoPointItemNumSave))
    (Variables|Default|SetNumWordsDelivered 0)
    (if (== (Variables|Default|GetNumPlayThroughs) (Variables|Default|GetMaxNumPlayThroughs))
      (Default|SpeakerDeliveredInformation (Variables|Default|GetSpeakerManager)))
    (else
      ;[1 1 1] Delivers information point at last position in array
      (Variables|Default|SetInfoItemToBeDelivered (Utilities|Array|Get(acopy) (Variables|Default|GetInfoPointItemNum) (Utilities|Array|LastIndex (Variables|Default|GetInfoPointItemNum))))
      (CallFunction|DeliverInfo (Variables|Default|GetWordList))
      ;[1 1 1] Removes last position point in array, reducing the size each run through
      (Utilities|Array|RemoveIndex (Variables|Default|GetInfoPointItemNum) (Utilities|Array|LastIndex (Variables|Default|GetInfoPointItemNum)))
      (Utilities|FlowControl|Delay (+ (Variables|Default|GetInfoDuration) 1.0))
      (Variables|Default|SetNumWordsDelivered (+ (Variables|Default|GetNumWordsDelivered) 1))
      (CallFunction|PlayThroughInformation))))

(event Custom|Create%20Random%20Word%20List%20Order
  (bind _infopointitemnum (Variables|Default|GetInfoPointItemNum))
  ;[1 1 1] Creates a 10 item array, randomises the order and resizes to required number of elements for trial
  (Utilities|Array|Shuffle (Variables|Default|GetInfoPointItemNum))
  (Utilities|Array|Resize _infopointitemnum (Variables|Default|GetList%20size))
  (Variables|Default|SetInfoPointItemNumSave _infopointitemnum))

(event Custom|AddLevelData
  (if (Variables|Default|GetUsesDataTable)
    (Utilities|FlowControl|Delay 0.1)))

(event Custom|Set%20Speaker%20Attributes
  (switch int (Variables|Default|GetSPK_MeshSelection)
    (:0
      _)
    (:1
      _)
    (:2
      (goto _label SPK%20Aesthetic%2002))
    (:3
      (goto _label SPK%20Aesthetic%2003))
    (:4
      (goto _label SPK%20Aesthetic%2004))
    (:5
      (goto _label SPK%20Aesthetic%2005))
    (:6
      (goto _label SPK%20Aesthetic%2006)))
  (Utilities|NewMacro0 :!label _label))

(event EventBeginPlay
  (Input|EnableInput (Game|GetPlayerController 0))
  (CallFunction|CreateRandomWordListOrder)
  (bind _returnvalue (Actor|GetActorOfClass "/Game/Blueprints/Environment/BP_Speaker_Gameplay_Base.BP_Speaker_Gameplay_Base_C"))
  (Variables|Default|SetSpeakerManager _returnvalue)
  (Utilities|FlowControl|Delay 1.0)
  (CallFunction|SetSpeakerAttributes))

(event EventPressButton
  (if (not (== (Variables|Default|GetNumPlayThroughs) (Variables|Default|GetMaxNumPlayThroughs)))
    (if (not (Variables|Default|GetIsPlaying?))
      (Variables|Default|SetIsPlaying? true)
      (Audio|PlaySoundatLocation "/Game/Sound/Environment/S_Confim_01.S_Confim_01" (Transformation|GetWorldLocation (Variables|Default|GetDefaultSceneRoot)) "0, 0, 0" 1.0 1.0 0.0 0 0 0)
      (Utilities|FlowControl|Delay 1.0)
      (Variables|Default|SetNumPlayThroughs (+ (Variables|Default|GetNumPlayThroughs) 1))
      (CallFunction|PlayThroughInformation))))

(fn ConstructionScript)

(fn DeliverInfo
  (params (InformationList :type Array%20of%20Sound%20Base%20Object%20References))
  (bind _infoitemtobedelivered (Variables|Default|GetInfoItemToBeDelivered))
  (bind _output (Utilities|Array|Get(acopy) InformationList _infoitemtobedelivered))
  (Audio|PlaySoundatLocation _output (Transformation|GetWorldLocation (Variables|Default|GetDefaultSceneRoot self)) "0, 0, 0" 2.5 1.0 0.0 "/Game/Sound/Attenuation/Attenuation_01.Attenuation_01" 0 0)
  (Variables|Default|SetInfoDuration (Variables|/Script/Engine.SoundBase|GetDuration _output)))