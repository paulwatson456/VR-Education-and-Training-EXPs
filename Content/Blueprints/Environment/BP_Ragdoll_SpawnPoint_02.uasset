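; Ragdoll spawn point actor that places a RagdollBP in one of three preset poses, keeping only one ragdoll alive at a time.
; Each spawn event destroys the tracked ragdoll and support box, then spawns at offsets from the root's relative location.
; Variants 01 and 02 share a location but differ in rotation, while 03 also spawns a support box.
; ReSpawnRagdoll destroys the current ragdoll and always reruns variant 03.
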(event Custom|Spawn%20Ragdoll%2001
  (Utilities|IsValid (Variables|Default|GetBoxSupport)
    (:Is%20Valid
      (Actor|DestroyActor (Variables|Default|GetBoxSupport)))
    (:Is%20Not%20Valid
      _))
  (Utilities|IsValid (Variables|Default|GetRagdollActor)
    (:Is%20Valid
      (Actor|DestroyActor (Variables|Default|GetRagdollActor)))
    (:Is%20Not%20Valid
      _))
  (bind _returnvalue (Game|SpawnActorfromClass "/Game/ContentPacks/Mannequin/Character/Mesh/RagdollBP.RagdollBP_C" (Math|Transform|MakeTransform (+ (Variables|Default|GetSpawn_01_LocationRelative) (Variables|/Script/Engine.SceneComponent|GetRelativeLocation (Variables|Default|GetDefaultSceneRoot))) (Variables|Default|GetSpawn%2001%20Rotation)) "Undefined" 0 0))
  (Variables|Default|SetRagdollActor _returnvalue))

(event Custom|ReSpawnRagdoll
  (Actor|DestroyActor (Variables|Default|GetRagdollActor))
  (CallFunction|SpawnRagdoll03))

(event Custom|SpawnRagdoll%2002
  (Utilities|IsValid (Variables|Default|GetBoxSupport)
    (:Is%20Valid
      (Actor|DestroyActor (Variables|Default|GetBoxSupport)))
    (:Is%20Not%20Valid
      _))
  (Utilities|IsValid (Variables|Default|GetRagdollActor)
    (:Is%20Valid
      (Actor|DestroyActor (Variables|Default|GetRagdollActor)))
    (:Is%20Not%20Valid
      _))
  (bind _returnvalue (Game|SpawnActorfromClass "/Game/ContentPacks/Mannequin/Character/Mesh/RagdollBP.RagdollBP_C" (Math|Transform|MakeTransform (+ (Variables|Default|GetSpawn_01_LocationRelative) (Variables|/Script/Engine.SceneComponent|GetRelativeLocation (Variables|Default|GetDefaultSceneRoot))) (Variables|Default|GetSpawn%2002%20Rotation)) "Undefined" 0 0))
  (Variables|Default|SetRagdollActor _returnvalue))

(event Custom|SpawnRagdoll%2003
  (Utilities|IsValid (Variables|Default|GetBoxSupport)
    (:Is%20Valid
      (Actor|DestroyActor (Variables|Default|GetBoxSupport)))
    (:Is%20Not%20Valid
      _))
  (Utilities|IsValid (Variables|Default|GetRagdollActor)
    (:Is%20Valid
      (Actor|DestroyActor (Variables|Default|GetRagdollActor)))
    (:Is%20Not%20Valid
      _))
  (bind _returnvalue (Game|SpawnActorfromClass "/Game/ContentPacks/Mannequin/Character/Mesh/RagdollBP.RagdollBP_C" (Math|Transform|MakeTransform (+ (Variables|/Script/Engine.SceneComponent|GetRelativeLocation (Variables|Default|GetDefaultSceneRoot)) (Variables|Default|GetSpawn_03_LocationRelative)) (Variables|Default|GetSpawn%2003%20Rotation)) "Undefined" 0 0))
  (Variables|Default|SetRagdollActor _returnvalue)
  (bind _returnvalue_2 (Game|SpawnActorfromClass "/Game/Mesh/SM_Box_01.SM_Box_01_C" (Math|Transform|MakeTransform (+ (Variables|/Script/Engine.SceneComponent|GetRelativeLocation (Variables|Default|GetDefaultSceneRoot)) (Variables|Default|GetSpawn_Box_03_LocationRelative)) (Variables|Default|GetSpawn%2003%20Box%20Rotation)) "Undefined" 0 0))
  (Variables|Default|SetBoxSupport _returnvalue_2))

(event EventBeginPlay)

(fn ConstructionScript)