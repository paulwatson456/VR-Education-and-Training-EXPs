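; BP_NumberFrame_WithContent is an environment frame that displays its FrameContent value through a UI_FrameNumber widget on a widget component.
; On BeginPlay it casts and caches the widget, then sets FrameText from FrameContent after a short delay.
; The SetFrameText event reapplies FrameContent to the cached widget on demand.
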(event Custom|Set%20Frame%20Text
  (Variables|/Game/Blueprints/UI/UI_FrameNumber.UI_FrameNumber_C|SetFrameText (Variables|Default|GetUI_Component) (Variables|Default|GetFrameContent)))

(event Collision|EventActorBeginOverlap
  (params (OtherActor :type Actor%20Object%20Reference)))

(event EventTick
  (params (DeltaSeconds :type Float%20%28single-precision%29)))

(event EventBeginPlay
  (bind _asui_frame_number (Utilities|Casting|CastToUI_FrameNumber (UserInterface|GetUserWidgetObject (Variables|Default|GetWidget))))
  (bind _output_get (Variables|Default|SetUI_Component _asui_frame_number))
  (Utilities|FlowControl|Delay 0.2)
  (Variables|/Game/Blueprints/UI/UI_FrameNumber.UI_FrameNumber_C|SetFrameText _output_get (Variables|Default|GetFrameContent)))

(fn ConstructionScript)