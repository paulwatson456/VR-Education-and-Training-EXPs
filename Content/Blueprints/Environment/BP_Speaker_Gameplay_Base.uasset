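; Base speaker gameplay actor that runs two speakers in turn during a speaker trial section.
; On BeginPlay it reads mesh and start position from the level attributes' data map, then selects SPK01's word list by enum switch.
; StartState powers the starting speaker, alternating on delivery callbacks until two deliveries power both off and notify the level director.
; A helper fills each speaker's attribute widget with mesh, position and voice/word-list labels.
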(event Custom|Set%20Speaker%20Attributes
  (Variables|/Game/Blueprints/Environment/BP_WordLogic_Base.BP_WordLogic_Base_C|SetSpeakerManager (Variables|Default|GetSPK%2001) self)
  (Variables|/Game/Blueprints/Environment/BP_WordLogic_Base.BP_WordLogic_Base_C|SetSpeakerManager (Variables|Default|GetSPK%2002) self))

(event Custom|Start%20State
  (CallFunction|PowerSwitches))

(event Custom|End%20State)

(event Custom|Speaker%20Delivered%20Information
  (bind _output_get (Variables|Default|SetNumberSpeakersDeliveredInfo (+ (Variables|Default|GetNumberSpeakersDeliveredInfo) 1)))
  (if (>= _output_get 2)
    (Default|PowerOFF (Variables|Default|GetSPK%2001%20Switch))
    (Class|BPIEventSectionEnd|EventSectionEnd(Message) (Variables|Default|GetLevelDirector))
    (else
      (CallFunction|PowerSwitches))))

(event Custom|Power%20Switches
  (switch int (Variables|Default|GetStarting%20Speaker)
    (:1
      (Default|PowerON (Variables|Default|GetSPK%2001%20Switch))
      (Variables|Default|SetStarting%20Speaker 2)
      (Default|PowerOFF (Variables|Default|GetSPK%2002%20Switch)))
    (:2
      (Default|PowerON (Variables|Default|GetSPK%2002%20Switch))
      (Variables|Default|SetStarting%20Speaker 1)
      (Default|PowerOFF (Variables|Default|GetSPK%2001%20Switch)))))

(event Custom|Set%20Attribute%20Display%20Data
  (bind (_spk_1_wordlist___voice _spk_2_wordlist___voice _spk_1_mesh _spk_2_mesh _starting_position) (CallFunction|NewFunction0 (Variables|/Game/Blueprints/Environment/BP_SetLevelAttributes_SPK_VAR.BP_SetLevelAttributes_SPK_VAR_C|GetTable%20Data%20Map (Variables|Default|GetLevelAttributes))))
  (CallFunction|NewFunction1 _spk_1_wordlist___voice _spk_1_mesh _starting_position _spk_2_wordlist___voice _spk_2_mesh _starting_position))

(event EventBeginPlay
  (Default|PowerOFF (Variables|Default|GetSPK%2001%20Switch))
  (bind _returnvalue (Actor|GetActorOfClass "/Game/Blueprints/Environment/BP_LvlDir_SPK_VAR_Trials.BP_LvlDir_SPK_VAR_Trials_C"))
  (Variables|Default|SetLevelDirector _returnvalue)
  (bind _returnvalue_2 (Actor|GetActorOfClass "/Game/Blueprints/Environment/BP_SetLevelAttributes_SPK_VAR.BP_SetLevelAttributes_SPK_VAR_C"))
  (Variables|Default|SetLevelAttributes _returnvalue_2)
  (Utilities|FlowControl|Delay 0.3)
  (bind (_spk_1_wordlist___voice _spk_2_wordlist___voice _spk_1_mesh _spk_2_mesh _starting_position) (CallFunction|NewFunction0 (Variables|/Game/Blueprints/Environment/BP_SetLevelAttributes_SPK_VAR.BP_SetLevelAttributes_SPK_VAR_C|GetTable%20Data%20Map (Variables|Default|GetLevelAttributes))))
  (Variables|Default|SetStarting%20Speaker _starting_position)
  (Variables|/Game/Blueprints/Environment/BP_WordLogic_Base.BP_WordLogic_Base_C|SetSPK_MeshSelection (Variables|Default|GetSPK%2001) _spk_1_mesh)
  (Variables|/Game/Blueprints/Environment/BP_WordLogic_Base.BP_WordLogic_Base_C|SetSPK_MeshSelection (Variables|Default|GetSPK%2002) _spk_2_mesh)
  (switch string (Variables|Default|GetNewVar_0)
    (:F1_1
      (Utilities|NewMacro0 (Variables|Default|GetSPK%2001) :!label _label
        (:NewParam9
          (CallFunction|SetSpeakerAttributes)
          (CallFunction|SetAttributeDisplayData))))
    (:F1_2
      (goto _label NewParam2))
    (:F1_3
      (goto _label NewParam3))
    (:F1_4
      (goto _label NewParam4))
    (:F1_5
      (goto _label NewParam5))
    (:F1_6
      (goto _label NewParam6))
    (:F1_7
      (goto _label NewParam7))
    (:F1_8
      (goto _label NewParam8))))

(fn ConstructionScript)

(fn NewFunction0
  (params (TargetMap :type Map%20of%20Strings%20to%20Strings))
  (bind _levelattributes (Variables|Default|GetLevelAttributes))
  (return (Utilities|String|Append (Utilities|String|Append (.Value (Utilities|Map|Find TargetMap (Variables|/Game/Blueprints/Environment/BP_SetLevelAttributes_SPK_VAR.BP_SetLevelAttributes_SPK_VAR_C|GetTrialSpeaker01Voice_ID _levelattributes))) "_") (.Value (Utilities|Map|Find TargetMap (Variables|/Game/Blueprints/Environment/BP_SetLevelAttributes_SPK_VAR.BP_SetLevelAttributes_SPK_VAR_C|GetTrialSpeaker01WordList_ID _levelattributes)))) (Utilities|String|Append (Utilities|String|Append (.Value (Utilities|Map|Find TargetMap (Variables|/Game/Blueprints/Environment/BP_SetLevelAttributes_SPK_VAR.BP_SetLevelAttributes_SPK_VAR_C|GetTrialSpeaker02Voice_ID _levelattributes))) "_") (.Value (Utilities|Map|Find TargetMap (Variables|/Game/Blueprints/Environment/BP_SetLevelAttributes_SPK_VAR.BP_SetLevelAttributes_SPK_VAR_C|GetTrialSpeaker02WordList_ID _levelattributes)))) (Math|Conversions|ToInteger(Byte) (.Value (Utilities|Map|Find TargetMap (Variables|/Game/Blueprints/Environment/BP_SetLevelAttributes_SPK_VAR.BP_SetLevelAttributes_SPK_VAR_C|GetTrialSpeaker01Look_ID _levelattributes)))) (Math|Conversions|ToInteger(Byte) (.Value (Utilities|Map|Find TargetMap (Variables|/Game/Blueprints/Environment/BP_SetLevelAttributes_SPK_VAR.BP_SetLevelAttributes_SPK_VAR_C|GetTrialSpeaker02Look_ID _levelattributes)))) (Math|Conversions|ToInteger(Byte) (.Value (Utilities|Map|Find TargetMap (Variables|/Game/Blueprints/Environment/BP_SetLevelAttributes_SPK_VAR.BP_SetLevelAttributes_SPK_VAR_C|GetTrialStartPosition_ID _levelattributes))))))

(fn NewFunction1
  (params (SPK%2001%20WordList :type String) (SPK%2001%20Mesh :type Integer) (SPK%2001%20Start%20Position :type Integer) (SPK%2002%20WordList :type String) (SPK%2002%20Mesh :type Integer) (SPK%2002%20Start%20Position :type Integer))
  (bind _asui_speaker_attributes (Utilities|Casting|CastToUI_SpeakerAttributes (UserInterface|GetWidget (Variables|/Game/Blueprints/Environment/BP_WordLogic_Base.BP_WordLogic_Base_C|GetW_SpeakerAttributes (Variables|Default|GetSPK%2001)))))
  (Variables|/Game/UI/3D_UI/UI_SpeakerAttributes.UI_SpeakerAttributes_C|SetMeshAttribute _asui_speaker_attributes (Utilities|Text|ToText(Integer) SPK%2001%20Mesh))
  (Variables|/Game/UI/3D_UI/UI_SpeakerAttributes.UI_SpeakerAttributes_C|SetStartPosAttribute _asui_speaker_attributes (Utilities|Text|ToText(Integer) SPK%2001%20Start%20Position))
  (Variables|/Game/UI/3D_UI/UI_SpeakerAttributes.UI_SpeakerAttributes_C|SetWordListAttribute _asui_speaker_attributes (Utilities|Text|ToText(String) SPK%2001%20WordList))
  (Variables|/Game/UI/3D_UI/UI_SpeakerAttributes.UI_SpeakerAttributes_C|SetRoomNumberAttribute _asui_speaker_attributes "")
  (bind _asui_speaker_attributes_2 (Utilities|Casting|CastToUI_SpeakerAttributes (UserInterface|GetWidget (Variables|/Game/Blueprints/Environment/BP_WordLogic_Base.BP_WordLogic_Base_C|GetW_SpeakerAttributes (Variables|Default|GetSPK%2002)))))
  (Variables|/Game/UI/3D_UI/UI_SpeakerAttributes.UI_SpeakerAttributes_C|SetMeshAttribute _asui_speaker_attributes_2 (Utilities|Text|ToText(Integer) SPK%2002%20Mesh))
  (Variables|/Game/UI/3D_UI/UI_SpeakerAttributes.UI_SpeakerAttributes_C|SetStartPosAttribute _asui_speaker_attributes_2 (Utilities|Text|ToText(Integer) SPK%2002%20Start%20Position))
  (Variables|/Game/UI/3D_UI/UI_SpeakerAttributes.UI_SpeakerAttributes_C|SetWordListAttribute _asui_speaker_attributes_2 (Utilities|Text|ToText(String) SPK%2002%20WordList))
  (Variables|/Game/UI/3D_UI/UI_SpeakerAttributes.UI_SpeakerAttributes_C|SetRoomNumberAttribute _asui_speaker_attributes_2 ""))