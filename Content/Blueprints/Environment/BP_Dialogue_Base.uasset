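; BP_Dialogue_Base is a dialogue Blueprint that plays sounds from an array in sequence, one track per LevelEventPlayAudio event.
; An AudioPlaying flag ignores further triggers until the sound's duration plus a short padding delay has elapsed.
; It then clears the flag, advances the track index with no bounds check, and notifies the LevelDirector that the level event is complete.
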(event EventLevelEventPlayAudio
  (if (not (Variables|Default|GetAudioPlaying?))
    (Audio|PlaySoundatLocation (Utilities|Array|Get(acopy) (Variables|Default|GetSoundArray) (Variables|Default|GetAudioTrackNumber)) "0, 0, 0" "0, 0, 0" 1.0 1.0 0.0 0 0 0)
    (Variables|Default|SetAudioPlaying? true)
    (Utilities|FlowControl|Delay (+ (Variables|/Script/Engine.SoundBase|GetDuration (Utilities|Array|Get(acopy) (Variables|Default|GetSoundArray) (Variables|Default|GetAudioTrackNumber))) 2.0))
    (Variables|Default|SetAudioPlaying? false)
    (Variables|Default|SetAudioTrackNumber (+ (Variables|Default|GetAudioTrackNumber) 1))
    (Class|INTLevelCommands|LevelEventComplete(Message) (Variables|Default|GetLevelDirector))))

(fn ConstructionScript)