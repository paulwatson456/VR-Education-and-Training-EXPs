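; BP_PowerPad_01 is an environment pad that shows and hides a button on a 3D title screen when its plate is overlapped.
; PowerOn and PowerOff toggle the plate's collision between query-only and none, switching overlap detection on and off.
; Overlap begin and end cast ActivationSource to UI_BP_TitleScreen_3D to call ShowButton or HideButton, without filtering the overlapping actor.
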(event OnComponentBeginOverlap(PlateCOL)
  (params (OverlappedComponent :type Primitive%20Component%20Object%20Reference) (OtherActor :type Actor%20Object%20Reference) (OtherComp :type Primitive%20Component%20Object%20Reference) (OtherBodyIndex :type Integer) (bFromSweep :type Boolean) (SweepResult :type Hit%20Result%20Structure%20%28by%20ref%29))
  (bind _asui_bp_title_screen_3d (Utilities|Casting|CastToUI_BP_TitleScreen_3D (Variables|Default|GetActivationSource)))
  (Default|ShowButton _asui_bp_title_screen_3d))

(event OnComponentEndOverlap(PlateCOL)
  (params (OverlappedComponent :type Primitive%20Component%20Object%20Reference) (OtherActor :type Actor%20Object%20Reference) (OtherComp :type Primitive%20Component%20Object%20Reference) (OtherBodyIndex :type Integer))
  (bind _asui_bp_title_screen_3d (Utilities|Casting|CastToUI_BP_TitleScreen_3D (Variables|Default|GetActivationSource)))
  (Default|HideButton _asui_bp_title_screen_3d))

(event Custom|PowerOn
  (Collision|SetCollisionEnabled (Variables|Default|GetPlateCOL) "QueryOnly"))

(event Custom|PowerOff
  (Collision|SetCollisionEnabled (Variables|Default|GetPlateCOL) "NoCollision"))

(event EventBeginPlay)

(fn ConstructionScript)