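; BP_LvlDir_SPK_VAR_Trials is a level director that sequences the SPK VAR trials level.
; On BeginPlay it finds the level attributes and speaker gameplay actors, then labels the left and right number frames by StartingPosition.
; A sequential, non-looping MultiGate advances per NextEventSection call through two delayed narrations, speaker gameplay start, another narration and level end.
; Player relocation logic in SetPlayerPostion is disconnected.
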(event Custom|Set%20Player%20Postion
  (if (== (Variables|/Game/Blueprints/Environment/BP_SetLevelAttributes_SPK_VAR.BP_SetLevelAttributes_SPK_VAR_C|GetStartingPosition (Variables|Default|GetSetLevelAttREF)) 1)
    (Variables|/Game/Blueprints/Environment/BP_NumberFrame_WithContent.BP_NumberFrame_WithContent_C|SetFrameContent (Variables|Default|GetLeft%20Number) "1")
    (Variables|/Game/Blueprints/Environment/BP_NumberFrame_WithContent.BP_NumberFrame_WithContent_C|SetFrameContent (Variables|Default|GetRight%20Number) "2")
    (else
      (Variables|/Game/Blueprints/Environment/BP_NumberFrame_WithContent.BP_NumberFrame_WithContent_C|SetFrameContent (Variables|Default|GetLeft%20Number) "2")
      (Variables|/Game/Blueprints/Environment/BP_NumberFrame_WithContent.BP_NumberFrame_WithContent_C|SetFrameContent (Variables|Default|GetRight%20Number) "1")))
  (Default|SetFrameText (Variables|Default|GetLeft%20Number))
  (Default|SetFrameText (Variables|Default|GetRight%20Number)))

(event EventBeginPlay
  (|CallParentFunction)
  (bind _returnvalue (Actor|GetActorOfClass "/Game/Blueprints/Environment/BP_SetLevelAttributes_SPK_VAR.BP_SetLevelAttributes_SPK_VAR_C"))
  (Variables|Default|SetSetLevelAttREF _returnvalue)
  (bind _returnvalue_2 (Actor|GetActorOfClass "/Game/Blueprints/Environment/BP_Speaker_Gameplay_Base.BP_Speaker_Gameplay_Base_C"))
  (Variables|Default|SetSpeakerGameplay _returnvalue_2)
  (Utilities|FlowControl|Delay 0.2)
  (CallFunction|SetPlayerPostion)
  (CallFunction|NextEventSection))

(event EventNextEventSection
  (CallFunction|NextEventCheck)
  (Utilities|FlowControl|MultiGate false false -1
    (:Out%200
      (Utilities|FlowControl|Delay 5.0)
      (Class|INTLevelCommands|LevelEventPlayAudio(Message) (Variables|Default|GetAudioNarrationBP_01)))
    (:Out%201
      (Utilities|FlowControl|Delay 1e+01)
      (Class|INTLevelCommands|LevelEventPlayAudio(Message) (Variables|Default|GetAudioNarrationBP_01)))
    (:Out%202
      (Default|StartState (Variables|Default|GetSpeakerGameplay)))
    (:Out%203
      (Utilities|FlowControl|Delay 3.0)
      (Class|INTLevelCommands|LevelEventPlayAudio(Message) (Variables|Default|GetAudioNarrationBP_01)))
    (:Out%204
      (CallFunction|LevelEndSPKVAR))))

(fn ConstructionScript
  (|CallParentFunction))