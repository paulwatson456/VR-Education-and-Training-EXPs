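; BP_WordLogic_Tutorial plays a randomised spoken word list for a tutorial trial.
; On BeginPlay it shuffles item indices, trims them to ListSize and saves the order.
; PressButton replays that order up to a maximum count, delivering sounds recursively from the array's end with duration-based delays, then notifies BP_SpeakerManager after the final playthrough.
; Every WordListID case uses WordList01; other list branches are disconnected.
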(event Custom|PlayThroughInformation
  (if (== (Variables|Default|GetList%20size) (Variables|Default|GetNumInfoDelivered))
    (Variables|Default|SetIsPlaying? false)
    (Variables|Default|SetInfoPointItemNum (Variables|Default|GetInfoPointItemNumSave))
    (Variables|Default|SetNumInfoDelivered 0)
    (if (== (Variables|Default|GetNumPlayThroughs) (Variables|Default|GetMaxNumPlayThroughs))
      (Default|DeliveredInfoPointEvent (Variables|Default|GetSpeakerManager)))
    (else
      ;[1 1 1] Delivers information point at last position in array
      (bind _output_get (Variables|Default|SetInfoItemToBeDelivered (Utilities|Array|Get(acopy) (Variables|Default|GetInfoPointItemNum) (Utilities|Array|LastIndex (Variables|Default|GetInfoPointItemNum)))))
      (Development|PrintString (Utilities|String|ToString(Integer) _output_get))
      (switch int (Variables|Default|GetWordListID)
        (:1
          _)
        (:2
          _)
        (:3
          _)
        (:4
          _)
        (:5
          _)
        (:6
          _)
        (:7
          _)
        (:8
          _)
        (:9
          _)
        (:10
          _)
        (:11
          _)
        (:12
          _)
        (:13
          _)
        (:14
          _)
        (:15
          _)
        (:16
          _))
      (CallFunction|DeliverInfo (Variables|Default|GetWordList_01))
      ;[1 1 1] Removes last position point in array, reducing the size each run through
      (Utilities|Array|RemoveIndex (Variables|Default|GetInfoPointItemNum) (Utilities|Array|LastIndex (Variables|Default|GetInfoPointItemNum)))
      (Utilities|FlowControl|Delay (+ (Variables|Default|GetInfoDuration) 1.0))
      (Variables|Default|SetNumInfoDelivered (+ (Variables|Default|GetNumInfoDelivered) 1))
      (CallFunction|PlayThroughInformation))))

(event EventBeginPlay
  (bind _infopointitemnum (Variables|Default|GetInfoPointItemNum))
  (bind _outactors (Actor|GetAllActorsOfClass "/Game/Blueprints/Environment/BP_SpeakerManager.BP_SpeakerManager_C"))
  (Variables|Default|SetSpeakerManager (Utilities|Array|Get(acopy) _outactors))
  (Input|EnableInput (Game|GetPlayerController 0))
  ;[1 1 1] Creates a 10 item array, randomises the order and resizes to required number of elements for trial
  (Utilities|Array|Shuffle (Variables|Default|GetInfoPointItemNum))
  (Utilities|Array|Resize _infopointitemnum (Variables|Default|GetList%20size))
  (Variables|Default|SetInfoPointItemNumSave _infopointitemnum))

(event EventPressButton
  (if (not (== (Variables|Default|GetNumPlayThroughs) (Variables|Default|GetMaxNumPlayThroughs)))
    (if (not (Variables|Default|GetIsPlaying?))
      (Variables|Default|SetIsPlaying? true)
      (Variables|Default|SetNumPlayThroughs (+ (Variables|Default|GetNumPlayThroughs) 1))
      (CallFunction|PlayThroughInformation))))

(event Input|KeyboardEvents|9
  (params (Key :type Key%20Structure :default "None"))
  (:Pressed
    (Development|PrintString (Utilities|String|ToString(Integer) (Utilities|Array|Length (Variables|Default|GetInfoPointItemNum))))))

(fn ConstructionScript)

(fn DeliverInfo
  (params (InformationList :type Array%20of%20Sound%20Base%20Object%20References))
  (bind _infoitemtobedelivered (Variables|Default|GetInfoItemToBeDelivered))
  (bind _output (Utilities|Array|Get(acopy) InformationList _infoitemtobedelivered))
  (Audio|PlaySoundatLocation _output "0, 0, 0" "0, 0, 0" 1.0 1.0 0.0 0 0 0)
  (Variables|Default|SetInfoDuration (Variables|/Script/Engine.SoundBase|GetDuration _output)))