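; BP_Target_01 is a moving target that awards points when something overlaps its collider.
; On BeginPlay it caches the score actor and its widget, which displays the point value.
; A hit passes points to BP_Target_Score_01, plays a sound and briefly flashes the widget red.
; Tick moves the base back and forth at per-axis speeds, using Delay nodes to toggle direction.
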(event OnComponentBeginOverlap(Target_Col)
  (params (OverlappedComponent :type Primitive%20Component%20Object%20Reference) (OtherActor :type Actor%20Object%20Reference) (OtherComp :type Primitive%20Component%20Object%20Reference) (OtherBodyIndex :type Integer) (bFromSweep :type Boolean) (SweepResult :type Hit%20Result%20Structure%20%28by%20ref%29))
  (bind _target_vis_ui (Variables|Default|GetTarget%20Vis%20UI))
  (Variables|/Game/Blueprints/Game_Target/BP_Target_Score_01.BP_Target_Score_01_C|SetPointsValue (Variables|Default|GetScoreREF) (Variables|Default|GetPoints))
  (Default|10Points (Variables|Default|GetScoreREF))
  (Appearance|SetColorandOpacity _target_vis_ui "(R=1.000000,G=0.074743,B=0.000000,A=1.000000)" :!class /Script/UMG.UserWidget)
  (Audio|PlaySoundatLocation "/Game/Sound/Game_Target/S_Target_Hit_01_Cue.S_Target_Hit_01_Cue" (Transformation|GetWorldLocation (Variables|Default|GetTarget_Base)) "0, 0, 0" 1.0 1.0 0.0 0 0 0)
  (Utilities|FlowControl|Delay 0.2)
  (Appearance|SetColorandOpacity _target_vis_ui "(R=1.000000,G=1.000000,B=1.000000,A=1.000000)" :!class /Script/UMG.UserWidget))

(event EventBeginPlay
  (bind _asbp_target_score_01 (Utilities|Casting|CastToBP_Target_Score_01 (Variables|Default|GetScore_Actor)))
  (Variables|Default|SetScoreREF _asbp_target_score_01)
  (bind _asui_g_target_vis_01 (Utilities|Casting|CastToUI_G_Target_Vis_01 (UserInterface|GetUserWidgetObject (Variables|Default|GetTarget_Visual_Widget))))
  (bind _output_get (Variables|Default|SetTarget%20Vis%20UI _asui_g_target_vis_01))
  (Variables|/Game/UI/Game_Target/UI_G_Target_Vis_01.UI_G_Target_Vis_01_C|SetPointsDisplay _output_get (Variables|Default|GetPoints)))

(event Collision|EventActorBeginOverlap
  (params (OtherActor :type Actor%20Object%20Reference)))

(event EventTick
  (params (DeltaSeconds :type Float%20%28single-precision%29))
  (bind _delay (Variables|Default|GetDelay))
  (Utilities|FlowControl|FlipFlop
    (:A
      _)
    (:B
      _))
  (if (Variables|Default|GetSwitch%20Direction)
    (Transformation|AddRelativeLocation (Variables|Default|GetTarget_Base) (Math|Vector|MakeVector (* DeltaSeconds (Variables|Default|GetX_Plus)) (* DeltaSeconds (Variables|Default|GetY_Plus)) (* DeltaSeconds (Variables|Default|GetZ_Plus))) false false)
    (Utilities|FlowControl|Delay _delay)
    (Variables|Default|SetSwitch%20Direction false)
    (else
      (Transformation|AddRelativeLocation (Variables|Default|GetTarget_Base) (Math|Vector|MakeVector (* DeltaSeconds (Variables|Default|GetX_Minus)) (* DeltaSeconds (Variables|Default|GetY_Minus)) (* DeltaSeconds (Variables|Default|GetZ_Minus))) false false)
      (Utilities|FlowControl|Delay _delay)
      (Variables|Default|SetSwitch%20Direction true))))

(fn ConstructionScript)