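; BP_Target_Score_01 is a target scoring Blueprint that adds points to the score held by its ScoreDisplayWidget.
; On BeginPlay it casts that component's user widget to UI_G_Target_Score_01 and caches it as WidgetUI.
; Custom events for three point tiers increment the widget's CurrentScore directly.
; The 10-point event adds the PointsValue variable, while the 20 and 50-point events use hard-coded amounts.
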(event Custom|10%20points
  (bind _widgetui (Variables|Default|GetWidgetUI))
  (Variables|/Game/UI/Game_Target/UI_G_Target_Score_01.UI_G_Target_Score_01_C|SetCurrentScore _widgetui (+ (Variables|/Game/UI/Game_Target/UI_G_Target_Score_01.UI_G_Target_Score_01_C|GetCurrentScore _widgetui) (Variables|Default|GetPointsValue))))

(event Custom|20%20Points
  (bind _widgetui (Variables|Default|GetWidgetUI))
  (Variables|/Game/UI/Game_Target/UI_G_Target_Score_01.UI_G_Target_Score_01_C|SetCurrentScore _widgetui (+ (Variables|/Game/UI/Game_Target/UI_G_Target_Score_01.UI_G_Target_Score_01_C|GetCurrentScore _widgetui) 20)))

(event Custom|50%20Points
  (bind _widgetui (Variables|Default|GetWidgetUI))
  (Variables|/Game/UI/Game_Target/UI_G_Target_Score_01.UI_G_Target_Score_01_C|SetCurrentScore _widgetui (+ (Variables|/Game/UI/Game_Target/UI_G_Target_Score_01.UI_G_Target_Score_01_C|GetCurrentScore _widgetui) 50)))

(event EventBeginPlay
  (bind _asui_g_target_score_01 (Utilities|Casting|CastToUI_G_Target_Score_01 (UserInterface|GetUserWidgetObject (Variables|Default|GetScore_Display_Widget))))
  (Variables|Default|SetWidgetUI _asui_g_target_score_01))

(fn ConstructionScript)