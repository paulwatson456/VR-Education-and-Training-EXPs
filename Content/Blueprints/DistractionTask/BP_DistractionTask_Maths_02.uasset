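; Timed maths distraction task that shows random arithmetic questions on a widget component until time runs out, then notifies the level director.
; Flow runs from an optional loading animation into StartChallenge, whose timer fires EndChallenge to show the completion screen.
; PressButton detects hovered answer buttons, then fades in a new MathsCalc question with shuffled answers, without checking correctness.
; MathsCalc picks addition, subtraction or multiplication; its division case is unreachable.
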(event Custom|End%20Challenge
  (bind _ui_mathsquestion (Variables|Default|GetUI_MathsQuestion))
  (Variables|Default|SetChallengOver? true)
  (if (not (Variables|Default|GetAnswerSelected))
    (Widget|SetVisibility (Variables|/Game/Blueprints/UI/UI_MathsQuestion1.UI_MathsQuestion1_C|GetBTN_Answer_01 (Variables|Default|GetUI_MathsQuestion)) "HitTestInvisible")
    (Widget|SetRenderOpacity (Variables|/Game/Blueprints/UI/UI_MathsQuestion1.UI_MathsQuestion1_C|GetMathsLayout (Variables|Default|GetUI_MathsQuestion)) 0.0)
    (Utilities|FlowControl|Delay 1.0)
    (Components|Animation|PlayAnimation _ui_mathsquestion (Variables|/Game/Blueprints/UI/UI_MathsQuestion1.UI_MathsQuestion1_C|GetANIM_CompleteFade _ui_mathsquestion) 0.0 1 "Reverse"
      (:then
        (Utilities|FlowControl|Delay 0.2)
        (Widget|SetRenderOpacity (Variables|/Game/Blueprints/UI/UI_MathsQuestion1.UI_MathsQuestion1_C|GetComplete _ui_mathsquestion) 1.0)
        (Utilities|FlowControl|Delay 2.0)
        (Widget|SetRenderOpacity (Variables|/Game/Blueprints/UI/UI_MathsQuestion1.UI_MathsQuestion1_C|GetComplete (Variables|Default|GetUI_MathsQuestion)) 0.0)
        (Widget|SetVisibility (Variables|Default|GetUI_MathsQuestion) "Visible")
        (Class|BPIEventSectionEnd|EventSectionEnd(Message) (Variables|Default|GetLevelDirector))))))

(event Custom|LoadingChallenge
  (bind _ui_mathsquestion (Variables|Default|GetUI_MathsQuestion))
  (bind _ui_mathsquestion_2 (Variables|Default|GetUI_MathsQuestion))
  (Variables|Default|SetIsLoading true)
  (Widget|SetRenderOpacity (Variables|/Game/Blueprints/UI/UI_MathsQuestion1.UI_MathsQuestion1_C|GetLoading (Variables|Default|GetUI_MathsQuestion)) 1.0)
  (Components|Animation|PlayAnimation _ui_mathsquestion (Variables|/Game/Blueprints/UI/UI_MathsQuestion1.UI_MathsQuestion1_C|GetANIM_LoadingFade _ui_mathsquestion) 0.0 3 "PingPong"
    (:Finished
      (Variables|Default|SetHasLoaded? true)
      (Utilities|FlowControl|Delay 1.0)
      (Components|Animation|PlayAnimation _ui_mathsquestion_2 (Variables|/Game/Blueprints/UI/UI_MathsQuestion1.UI_MathsQuestion1_C|GetANIM_LoadingFade _ui_mathsquestion_2) 0.0
        (:then
          (Utilities|FlowControl|Delay 1.0)
          (CallFunction|ChallengeNextSequence))))))

(event Custom|ClearScreen
  (Widget|SetRenderOpacity (Variables|/Game/Blueprints/UI/UI_MathsQuestion1.UI_MathsQuestion1_C|GetMathsLayout (Variables|Default|GetUI_MathsQuestion)) 0.0)
  (Widget|SetVisibility (Variables|Default|GetUI_MathsQuestion) "HitTestInvisible"))

(event Custom|ChallengeNextSequence
  (if (Variables|Default|GetHasLoaded?)
    (CallFunction|StartChallenge)
    (else
      (CallFunction|LoadingChallenge))))

(event Custom|DescribeChallenge
  (Variables|Default|SetDescribing true)
  (Components|Animation|PlayAnimation (Variables|Default|GetUITarget) (Variables|/Game/Blueprints/UI/UI_MathsQuestion.UI_MathsQuestion_C|GetAnim_Description_FadeIn (Variables|Default|GetUITarget)) 0.0
    (:Finished
      (Utilities|FlowControl|Delay 2.0)
      (Components|Animation|PlayAnimation (Variables|Default|GetUITarget) (Variables|/Game/Blueprints/UI/UI_MathsQuestion.UI_MathsQuestion_C|GetAnim_Description_FadeIn (Variables|Default|GetUITarget)) 0.0 1 "Reverse"
        (:Finished
          (Variables|Default|SetDescriptionShown? true)
          (CallFunction|ChallengeNextSequence))))))

(event Custom|FadeText
  (Components|Animation|PlayAnimation (Variables|Default|GetUITarget) (Variables|/Game/Blueprints/UI/UI_MathsQuestion.UI_MathsQuestion_C|GetAnim_AllFadeOUT (Variables|Default|GetUITarget)) 0.0))

(event Custom|Start%20Challenge
  (bind _ui_mathsquestion (Variables|Default|GetUI_MathsQuestion))
  (Utilities|Time|SetTimerbyEvent (delegate Custom|End%20Challenge) 1e+01)
  (Components|Animation|PlayAnimation _ui_mathsquestion (Variables|/Game/Blueprints/UI/UI_MathsQuestion1.UI_MathsQuestion1_C|GetANIM_AllMathsFade _ui_mathsquestion) 0.0 1 "Reverse"
    (:then
      (Utilities|FlowControl|Delay 0.2)
      (Widget|SetRenderOpacity (Variables|/Game/Blueprints/UI/UI_MathsQuestion1.UI_MathsQuestion1_C|GetMathsLayout _ui_mathsquestion) 1.0)
      (Widget|SetVisibility (Variables|Default|GetUI_MathsQuestion) "Visible"))))

(event EventBeginPlay
  (Input|EnableInput (Game|GetPlayerController 0))
  (bind _asui_maths_question_1 (Utilities|Casting|CastToUI_MathsQuestion1 (UserInterface|GetUserWidgetObject (Variables|Default|GetWidget_Maths%20Question))))
  (Variables|Default|SetUI_MathsQuestion _asui_maths_question_1)
  (bind (_number01 _number02 _numbercalc _numberanswer01 _numberanswer02 _numberanswer03) (CallFunction|MathsCalc))
  (CallFunction|SetUIfromMathsCalc (Variables|Default|GetUI_MathsQuestion) _number01 _number02 _numbercalc _numberanswer01 _numberanswer02 _numberanswer03)
  (CallFunction|ClearScreen)
  (bind _outactors (Actor|GetAllActorsOfClass "/Game/Blueprints/Environment/BP_LvlDir_LevelSelect.BP_LvlDir_LevelSelect_C"))
  (Variables|Default|SetLevelDirector (Utilities|Array|Get(acopy) _outactors)))

(event EventChallengeComms
  (CallFunction|StartChallenge))

(event EventPressButton
  (bind _ui_mathsquestion (Variables|Default|GetUI_MathsQuestion))
  (bind _ui_mathsquestion_2 (Variables|Default|GetUI_MathsQuestion))
  (bind _ui_mathsquestion_3 (Variables|Default|GetUI_MathsQuestion))
  (Variables|Default|SetAnswerSelected true)
  (if (not (Variables|Default|GetChallengOver?))
    (if (Math|Boolean|ORBoolean (Widget|IsHovered (Variables|/Game/Blueprints/UI/UI_MathsQuestion1.UI_MathsQuestion1_C|GetBTN_Answer_01 _ui_mathsquestion)) (Widget|IsHovered (Variables|/Game/Blueprints/UI/UI_MathsQuestion1.UI_MathsQuestion1_C|GetBTN_Answer_02 _ui_mathsquestion)) (Widget|IsHovered (Variables|/Game/Blueprints/UI/UI_MathsQuestion1.UI_MathsQuestion1_C|GetBTN_Answer_03 _ui_mathsquestion)))
      (Widget|SetVisibility (Variables|/Game/Blueprints/UI/UI_MathsQuestion1.UI_MathsQuestion1_C|GetBTN_Answer_01 (Variables|Default|GetUI_MathsQuestion)) "HitTestInvisible")
      (Components|Animation|PlayAnimation _ui_mathsquestion_2 (Variables|/Game/Blueprints/UI/UI_MathsQuestion1.UI_MathsQuestion1_C|GetANIM_AllMathsFade _ui_mathsquestion_2) 0.0
        (:Finished
          (bind (_number01 _number02 _numbercalc _numberanswer01 _numberanswer02 _numberanswer03) (CallFunction|MathsCalc))
          (bind _output_get (Variables|Default|SetNumberAnswers (Utilities|Array|MakeArray _numberanswer01 _numberanswer02 _numberanswer03)))
          (Utilities|Array|Shuffle _output_get)
          (CallFunction|SetUIfromMathsCalc (Variables|Default|GetUI_MathsQuestion) _number01 _number02 _numbercalc (Utilities|Array|Get(acopy) (Variables|Default|GetNumberAnswers)) (Utilities|Array|Get(acopy) (Variables|Default|GetNumberAnswers) 1) (Utilities|Array|Get(acopy) (Variables|Default|GetNumberAnswers) 2))
          (Components|Animation|PlayAnimation _ui_mathsquestion_3 (Variables|/Game/Blueprints/UI/UI_MathsQuestion1.UI_MathsQuestion1_C|GetANIM_AllMathsFade _ui_mathsquestion_3) 0.0 1 "Reverse"
            (:Finished
              (Widget|SetVisibility (Variables|/Game/Blueprints/UI/UI_MathsQuestion1.UI_MathsQuestion1_C|GetBTN_Answer_01 (Variables|Default|GetUI_MathsQuestion)) "Visible")
              (Variables|Default|SetAnswerSelected false)
              (if (Variables|Default|GetChallengOver?)
                (CallFunction|EndChallenge)))))))))

(event Input|KeyboardEvents|1
  (params (Key :type Key%20Structure :default "None"))
  (:Pressed
    (CallFunction|StartChallenge)))

(fn ConstructionScript)

(fn MathsCalc
  (switch int (Math|Random|RandomInteger 3)
    (:0
      (LocalVariables|SetNumber_01 (Math|Random|RandomInteger 10))
      (LocalVariables|SetNumber_02 (Math|Random|RandomInteger 10))
      (LocalVariables|SetCalculationAnswer (+ (LocalVariables|GetNumber_01) (LocalVariables|GetNumber_02)))
      (LocalVariables|SetNumber_01_Text (Utilities|Text|ToText(Integer) (LocalVariables|GetNumber_01)))
      (LocalVariables|SetNumber_02_Text (Utilities|Text|ToText(Integer) (LocalVariables|GetNumber_02)))
      (LocalVariables|SetNumberCalcText "+")
      (LocalVariables|SetNumberAnswerText_01 (Utilities|Text|ToText(Integer) (LocalVariables|GetCalculationAnswer)))
      (LocalVariables|SetNumberAnswerText_02 (Utilities|Text|ToText(Integer) (+ (LocalVariables|GetCalculationAnswer) (Math|Random|RandomIntegerinRange 1 12))))
      (LocalVariables|SetNumberAnswerText_03 (Utilities|Text|ToText(Integer) (- (LocalVariables|GetCalculationAnswer) (Math|Random|RandomIntegerinRange 1 12)))))
    (:1
      (LocalVariables|SetNumber_01 (Math|Random|RandomInteger 10))
      (LocalVariables|SetNumber_02 (Math|Random|RandomInteger 10))
      (LocalVariables|SetCalculationAnswer (- (LocalVariables|GetNumber_01) (LocalVariables|GetNumber_02)))
      (LocalVariables|SetNumber_01_Text (Utilities|Text|ToText(Integer) (LocalVariables|GetNumber_01)))
      (LocalVariables|SetNumber_02_Text (Utilities|Text|ToText(Integer) (LocalVariables|GetNumber_02)))
      (LocalVariables|SetNumberCalcText "-")
      (LocalVariables|SetNumberAnswerText_01 (Utilities|Text|ToText(Integer) (LocalVariables|GetCalculationAnswer)))
      (LocalVariables|SetNumberAnswerText_02 (Utilities|Text|ToText(Integer) (+ (LocalVariables|GetCalculationAnswer) (Math|Random|RandomIntegerinRange 1 12))))
      (LocalVariables|SetNumberAnswerText_03 (Utilities|Text|ToText(Integer) (- (LocalVariables|GetCalculationAnswer) (Math|Random|RandomIntegerinRange 1 12)))))
    (:2
      (LocalVariables|SetNumber_01 (Math|Random|RandomInteger 10))
      (LocalVariables|SetNumber_02 (Math|Random|RandomInteger 10))
      (LocalVariables|SetCalculationAnswer (* (LocalVariables|GetNumber_01) (LocalVariables|GetNumber_02)))
      (LocalVariables|SetNumber_01_Text (Utilities|Text|ToText(Integer) (LocalVariables|GetNumber_01)))
      (LocalVariables|SetNumber_02_Text (Utilities|Text|ToText(Integer) (LocalVariables|GetNumber_02)))
      (LocalVariables|SetNumberCalcText "X")
      (LocalVariables|SetNumberAnswerText_01 (Utilities|Text|ToText(Integer) (LocalVariables|GetCalculationAnswer)))
      (LocalVariables|SetNumberAnswerText_02 (Utilities|Text|ToText(Integer) (+ (LocalVariables|GetCalculationAnswer) (Math|Random|RandomIntegerinRange 1 12))))
      (LocalVariables|SetNumberAnswerText_03 (Utilities|Text|ToText(Integer) (- (LocalVariables|GetCalculationAnswer) (Math|Random|RandomIntegerinRange 1 12)))))
    (:3
      (LocalVariables|SetNumber_01 (Math|Random|RandomInteger 10))
      (LocalVariables|SetNumber_02 (Math|Random|RandomInteger 10))
      (LocalVariables|SetCalculationAnswer (/ (LocalVariables|GetNumber_01) (LocalVariables|GetNumber_02)))
      (LocalVariables|SetNumber_01_Text (Utilities|Text|ToText(Integer) (LocalVariables|GetNumber_01)))
      (LocalVariables|SetNumber_02_Text (Utilities|Text|ToText(Integer) (LocalVariables|GetNumber_02)))
      (LocalVariables|SetNumberCalcText "/")
      (LocalVariables|SetNumberAnswerText_01 (Utilities|Text|ToText(Integer) (LocalVariables|GetCalculationAnswer)))
      (LocalVariables|SetNumberAnswerText_02 (Utilities|Text|ToText(Integer) (+ (LocalVariables|GetCalculationAnswer) (Math|Random|RandomIntegerinRange 1 12))))
      (LocalVariables|SetNumberAnswerText_03 (Utilities|Text|ToText(Integer) (- (LocalVariables|GetCalculationAnswer) (Math|Random|RandomIntegerinRange 1 12))))))
  (return (LocalVariables|GetNumber_01_Text) (LocalVariables|GetNumber_02_Text) (LocalVariables|GetNumberCalcText) (LocalVariables|GetNumberAnswerText_01) (LocalVariables|GetNumberAnswerText_02) (LocalVariables|GetNumberAnswerText_03)))

(fn SetUIfromMathsCalc
  (params (UI_MathsQuestion :type UI%20Maths%20Question%201%20Object%20Reference) (UI_Number01 :type Text) (UI_Number02 :type Text) (UI_NumberCalc :type Text) (UI_NumberAnswer :type Text) (UI_NumberAnswerWrong01 :type Text) (UI_NumberAnswerWrong02 :type Text))
  (Variables|/Game/Blueprints/UI/UI_MathsQuestion1.UI_MathsQuestion1_C|SetUINumber01 UI_MathsQuestion UI_Number01)
  (Variables|/Game/Blueprints/UI/UI_MathsQuestion1.UI_MathsQuestion1_C|SetUINumber02 UI_MathsQuestion UI_Number02)
  (Variables|/Game/Blueprints/UI/UI_MathsQuestion1.UI_MathsQuestion1_C|SetUINumberCalc UI_MathsQuestion UI_NumberCalc)
  (Variables|/Game/Blueprints/UI/UI_MathsQuestion1.UI_MathsQuestion1_C|SetUINumberAnswer UI_MathsQuestion UI_NumberAnswer)
  (Variables|/Game/Blueprints/UI/UI_MathsQuestion1.UI_MathsQuestion1_C|SetUINumberAnswerWrong01 UI_MathsQuestion UI_NumberAnswerWrong01)
  (Variables|/Game/Blueprints/UI/UI_MathsQuestion1.UI_MathsQuestion1_C|SetUINumberAnswerWrong02 UI_MathsQuestion UI_NumberAnswerWrong02))