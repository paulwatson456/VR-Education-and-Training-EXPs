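; Demonstrator character Blueprint that plays a stepped, voiced demonstration with two skeletal meshes, a helper and a recovery man.
; BeginPlay sets starting animations and binds the next and previous switch events to StepForward and StepBackward.
; Each step moves a clamped counter that indexes parallel animation and sound arrays, replacing the current audio with sound attached to the helper.
; Forward steps loop animations, backward steps play once; input-enabling and reverse-playback nodes never run.
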(event Custom|StepBackward
  (if (Utilities|IsValid (Variables|Default|GetAudioComp))
    ;[1 1 1] Stops audio on button press
    (Audio|Components|Audio|Stop (Variables|Default|GetAudioComp)))
  (bind _output_get (Variables|Components|SetStepCounter (Math|Integer|Clamp(Integer) (- (Variables|Components|GetStepCounter) 1) 0 9)))
  (Components|Animation|PlayAnimation (Variables|Default|GetRP-Helper-Skel) (Utilities|Array|Get(acopy) (Variables|Default|GetRP_HELPER_AnimSequence_VoicAndAction_LOOP) _output_get) false)
  ;[0 1 0.1026] Array of Sounds
  (bind _returnvalue (Audio|SpawnSoundAttached (Utilities|Array|Get(acopy) (Variables|Default|GetRP-Audio-Sequence_VoiceAndAction) _output_get) (Variables|Default|GetRP-Helper-Skel) "None" "0, 0, 0" "0, 0, 0" "KeepRelativeOffset" false 1.0 1.0 0.0 0 0))
  (Variables|Default|SetAudioComp _returnvalue)
  ;[0 0.004862 1] RECOVERY MAN ANIMATIONS
  ;;[1 0.05117 0.09097] Array of animations
  (Components|Animation|PlayAnimation (Variables|Default|GetRP-Recovery-Skel) (Utilities|Array|Get(acopy) (Variables|Default|GetRP_RECOVERY_AnimSequence_VoicAndAction_LOOP) _output_get) false))

(event Custom|StepForward
  (Variables|Components|SetStepCounter (Math|Integer|Clamp(Integer) (+ (Variables|Components|GetStepCounter) 1) 0 9))
  (if (Utilities|IsValid (Variables|Default|GetAudioComp))
    (Audio|Components|Audio|Stop (Variables|Default|GetAudioComp)))
  (Components|Animation|PlayAnimation (Variables|Default|GetRP-Helper-Skel) (Utilities|Array|Get(acopy) (Variables|Default|GetRP_HELPER_AnimSequence_VoicAndAction_LOOP) (Variables|Components|GetStepCounter)) true)
  ;[0 1 0.1026] Array of Sounds
  (bind _returnvalue (Audio|SpawnSoundAttached (Utilities|Array|Get(acopy) (Variables|Default|GetRP-Audio-Sequence_VoiceAndAction) (Variables|Components|GetStepCounter)) (Variables|Default|GetRP-Helper-Skel) "None" "0, 0, 0" "0, 0, 0" "KeepRelativeOffset" false 1.0 1.0 0.0 0 0))
  (Variables|Default|SetAudioComp _returnvalue)
  ;[0 0.004862 1] RECOVERY MAN ANIMATIONS
  ;;[1 0.05117 0.09097] Array of animations
  (Components|Animation|PlayAnimation (Variables|Default|GetRP-Recovery-Skel) (Utilities|Array|Get(acopy) (Variables|Default|GetRP_RECOVERY_AnimSequence_VoicAndAction_LOOP) (Variables|Components|GetStepCounter)) true))

(event EventBeginPlay
  ;[1 1 1] Sets animation pose on begin play
  (Components|Animation|PlayAnimation (Variables|Default|GetRP-Recovery-Skel) "/Game/Animations/Recovery/RP-Recovery-Skel_Anim00-SP.RP-Recovery-Skel_Anim00-SP" false)
  (Components|Animation|PlayAnimation (Variables|Default|GetRP-Helper-Skel) "/Game/Animations/Helper/RP-Helper-Skel_Anim00-SP.RP-Helper-Skel_Anim00-SP" false)
  (EventDispatchers|BindEventtoNextStep (Variables|Default|GetSwitchNext) (delegate Custom|StepForward))
  (EventDispatchers|BindEventtoPreviousStep (Variables|Default|GetSwitchPrevious) (delegate Custom|StepBackward)))

(fn ConstructionScript)

(fn OnRepStepCounter)